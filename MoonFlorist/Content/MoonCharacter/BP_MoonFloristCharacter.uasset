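; Player character for Moon Florist that picks up flower-shop orders and drives the order list on the HUD.
; E, when collection is allowed, pulls a random row from the order DataTable, shows its description and resets the objective count.
; F is a test completion key that decrements the count and rebuilds the text through CompleteObjective using the row's keywords and colours.
; Tab flip-flops the order list's pull-out animation.
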(event `self.ReceiveBeginPlay`
  (bind _asbp_moon_florist_hud (cast `/Game/BP_MoonFloristHUD` (`PlayerController.GetHUD` (`GameplayStatics.GetPlayerController` 0))))
  (set `self.HUD` _asbp_moon_florist_hud)
  (set `self.HasOrder` false))

(event `Key|E`
  (params (Key :type "Key Structure"))
  (bind _returnvalue (`KismetMathLibrary.RandomIntegerInRange` 0 1))
  (:`Pressed`
    (if (`self.CanCollectOrder`)
      (`KismetSystemLibrary.PrintString` (`KismetStringLibrary.Conv_IntToString` _returnvalue))
      (bind _output_get (set `self.CurrentOrder` (`|GetArrayItem` (`self.RowTableName`) _returnvalue)))
      (bind _returnvalue_2 (`|GetDataTableRow` "/Game/User_Interface/OrderList/OrderListTable.OrderListTable" _output_get)
        (:`then`
          (set `self.HasOrder` true)
          (`RichTextBlock.SetText` (`/Game/User_Interface/OrderList/OrderList_Widget.DescriptionRichText` (`/Game/BP_MoonFloristHUD.OrderListUI` (`self.HUD`))) (`/Game/User_Interface/OrderList/OL_Lib.To Target Text` (`.OrderDiscription_21_27B4F049401D68C92D1C38BB64D1FA6E` (break `/Game/User_Interface/OrderList/OrderListStructure` _returnvalue_2))))
          (`Widget.SetVisibility` (`/Game/User_Interface/OrderList/OrderList_Widget.PressEtoRecieveOrder` (`/Game/BP_MoonFloristHUD.OrderListUI` (`self.HUD`))) "Hidden")
          (set `self.Count` 3))))))

(event `Key|F`
  (params (Key :type "Key Structure"))
  ;[1 1 1] Complete Order Testing
  (:`Pressed`
    (bind _result (`/Engine/EditorBlueprintResources/StandardMacros.DecrementInt` (`self.Count`))
      (:`  `
        (bind _returnvalue (`|GetDataTableRow` "/Game/User_Interface/OrderList/OrderListTable.OrderListTable" (`self.CurrentOrder`))
          (:`then`
            (bind (_orderdiscription _keyword1 _keyword2 _keyword3 _kwcolour1 _kwcolour2 _kwcolour3) (break `/Game/User_Interface/OrderList/OrderListStructure` _returnvalue))
            (bind _out_text (`/Game/User_Interface/OrderList/OL_Lib.CompleteObjective` _orderdiscription _keyword1 _keyword2 _keyword3 _result _kwcolour1 _kwcolour2 _kwcolour3))
            (`RichTextBlock.SetText` (`/Game/User_Interface/OrderList/OrderList_Widget.DescriptionRichText` (`/Game/BP_MoonFloristHUD.OrderListUI` (`self.HUD`))) (`/Game/User_Interface/OrderList/OL_Lib.To Target Text` _out_text))))))))

(event `Key|Tab`
  (params (Key :type "Key Structure"))
  (bind _orderlistui (`/Game/BP_MoonFloristHUD.OrderListUI` (`self.HUD`)))
  (bind _orderlistui_2 (`/Game/BP_MoonFloristHUD.OrderListUI` (`self.HUD`)))
  ;[1 1 1] Play Animation For OrderList
  (:`Pressed`
    (`/Engine/EditorBlueprintResources/StandardMacros.FlipFlop`
      (:`A`
        (`UserWidget.PlayAnimation` _orderlistui (`/Game/User_Interface/OrderList/OrderList_Widget.PullOutAnimation` _orderlistui) 0.0 1 "Reverse" 2.5))
      (:`B`
        (`UserWidget.PlayAnimation` _orderlistui_2 (`/Game/User_Interface/OrderList/OrderList_Widget.PullOutAnimation` _orderlistui_2) 0.0 1 "Forward" 2.5)))))

(fn `UserConstructionScript`)