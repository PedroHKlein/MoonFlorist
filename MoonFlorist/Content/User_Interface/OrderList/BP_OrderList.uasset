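; BP_OrderList is a world actor where the Moon Florist player can collect an order.
; Its Box component detects a BP_MoonFloristCharacter entering or leaving, showing or hiding the "Press E to receive order" prompt in the character's HUD OrderListUI.
; The same overlaps toggle the character's CanCollectOrder flag; the collection itself is not handled in this Blueprint.
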(event `self.ReceiveBeginPlay`)

(event `self.Box.OnComponentBeginOverlap`
  (params (OverlappedComponent :type "PrimitiveComponent Object Reference") (OtherActor :type "Actor Object Reference") (OtherComp :type "PrimitiveComponent Object Reference") (OtherBodyIndex :type Integer) (bFromSweep :type Boolean) (SweepResult :type "HitResult Structure (by ref)"))
  (bind _asbp_moon_florist_character (cast `/Game/BP_MoonFloristCharacter` OtherActor))
  (`Widget.SetVisibility` (`/Game/User_Interface/OrderList/OrderList_Widget.PressEtoRecieveOrder` (`/Game/BP_MoonFloristHUD.OrderListUI` (`/Game/BP_MoonFloristCharacter.HUD` _asbp_moon_florist_character))) "Visible")
  (set `/Game/BP_MoonFloristCharacter.CanCollectOrder` true _asbp_moon_florist_character))

(event `self.Box.OnComponentEndOverlap`
  (params (OverlappedComponent :type "PrimitiveComponent Object Reference") (OtherActor :type "Actor Object Reference") (OtherComp :type "PrimitiveComponent Object Reference") (OtherBodyIndex :type Integer))
  (bind _asbp_moon_florist_character (cast `/Game/BP_MoonFloristCharacter` OtherActor))
  (`Widget.SetVisibility` (`/Game/User_Interface/OrderList/OrderList_Widget.PressEtoRecieveOrder` (`/Game/BP_MoonFloristHUD.OrderListUI` (`/Game/BP_MoonFloristCharacter.HUD` _asbp_moon_florist_character))) "Hidden")
  (set `/Game/BP_MoonFloristCharacter.CanCollectOrder` false _asbp_moon_florist_character))

(fn `UserConstructionScript`)