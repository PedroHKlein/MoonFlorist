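; Player character for a florist game, handling interaction with the market, order board, arranging table, storage, radio and planters.
; E runs a raycast and distance check, then most stations FlipFlop the camera, input lock and HUD.
; Orders are picked randomly from a DataTable; F test-completes keywords, Tab/Z slides the list.
; Planter buttons cycle hologram flowers, consume stock, animate the hatch through timed growth, and add harvests to inventory.
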(event `Key|E`
  (params (Key :type "Key Structure"))
  (bind _returnvalue (`GameplayStatics.GetPlayerController` 0))
  (bind _returnvalue_2 (`GameplayStatics.GetPlayerController` 0))
  (:`Pressed`
    (bind (_returnvalue_3 _hitactor) (`self.InteractionCheck`))
    (bind _asbp_market (cast `/Game/Interactables/BP_Market` _hitactor))
    (if _returnvalue_3
      (`/Engine/EditorBlueprintResources/StandardMacros.FlipFlop`
        (:`A`
          (`PlayerController.SetViewTargetWithBlend` _returnvalue _asbp_market 1.0 "VTBlend_Linear" 0.0 false)
          (`Controller.SetIgnoreMoveInput` _returnvalue true)
          (`Controller.SetIgnoreLookInput` _returnvalue true)
          (set `PlayerController.bShowMouseCursor` true (`GameplayStatics.GetPlayerController` 0))
          (`MoonFloristHUD.ToggleAlpha` (`self.HUD`) true))
        (:`B`
          (`PlayerController.SetViewTargetWithBlend` (`GameplayStatics.GetPlayerController` 0) (`GameplayStatics.GetPlayerCharacter` 0) 1.0 "VTBlend_Linear" 0.0 false)
          (`Controller.ResetIgnoreMoveInput` _returnvalue_2)
          (`Controller.ResetIgnoreLookInput` _returnvalue_2)
          (set `PlayerController.bShowMouseCursor` false _returnvalue_2)
          (`WidgetBlueprintLibrary.SetFocusToGameViewport`)
          (`MoonFloristHUD.ToggleAlpha` (`self.HUD`) false))))))

(event `self.ReceiveBeginPlay`
  ;[1 1 1] Event Begin
  (bind _asbp_moon_florist_hud (cast `/Game/BP_MoonFloristHUD` (`PlayerController.GetHUD` (`GameplayStatics.GetPlayerController` 0))))
  (set `self.HUD` _asbp_moon_florist_hud)
  (set `self.HasOrder` false)
  (bind _asbp_moon_florist_character (cast `/Game/BP_MoonFloristCharacter` (`Controller.K2_GetPawn` (`GameplayStatics.GetPlayerController` 0))))
  (set `/Game/BP_MoonFloristCharacter.Player` null _asbp_moon_florist_character))

(event `Key|E`
  (params (Key :type "Key Structure"))
  (bind _returnvalue (`KismetMathLibrary.RandomIntegerInRange` 0 1))
  ;[0 0 0] OrderList Interaction
  (:`Pressed`
    (bind (_returnvalue_2 _hitactor) (`self.InteractionCheck`))
    (cast `/Game/Interactables/BP_OrderList` _hitactor)
    (if _returnvalue_2
      (`KismetSystemLibrary.PrintString` (`KismetStringLibrary.Conv_IntToString` _returnvalue))
      (bind _output_get (set `self.CurrentOrder` (`|GetArrayItem` (`self.RowTableName`) _returnvalue)))
      (bind _returnvalue_3 (`|GetDataTableRow` "/Game/User_Interface/OrderList/OrderListTable.OrderListTable" _output_get)
        (:`then`
          (set `self.HasOrder` true)
          (`RichTextBlock.SetText` (`/Game/User_Interface/OrderList/OrderList_Widget.DescriptionRichText` (`/Game/BP_MoonFloristHUD.OrderListUI` (`self.HUD`))) (`/Game/User_Interface/OrderList/OL_Lib.To Target Text` (`.OrderDiscription_21_27B4F049401D68C92D1C38BB64D1FA6E` (break `/Game/User_Interface/OrderList/OrderListStructure` _returnvalue_3))))
          (set `self.Count` 3))))))

(event `Key|E`
  (params (Key :type "Key Structure"))
  (bind _returnvalue (`GameplayStatics.GetPlayerController` 0))
  (bind _returnvalue_2 (`GameplayStatics.GetPlayerController` 0))
  ;[0 0 0] Interaction for Table - Flower Arranging
  (:`Pressed`
    (bind (_returnvalue_3 _hitactor) (`self.InteractionCheck`))
    (bind _asbp_flower_arrange_table (cast `/Game/Interactables/BP_FlowerArrangeTable` _hitactor))
    (if _returnvalue_3
      (`/Engine/EditorBlueprintResources/StandardMacros.FlipFlop`
        (:`A`
          (`PlayerController.SetViewTargetWithBlend` _returnvalue _asbp_flower_arrange_table 1.0 "VTBlend_Linear" 0.0 false)
          (`Controller.SetIgnoreMoveInput` _returnvalue true)
          (`Controller.SetIgnoreLookInput` _returnvalue true)
          (set `PlayerController.bShowMouseCursor` true (`GameplayStatics.GetPlayerController` 0))
          (`MoonFloristHUD.ToggleAlpha` (`self.HUD`) true))
        (:`B`
          (`PlayerController.SetViewTargetWithBlend` (`GameplayStatics.GetPlayerController` 0) (`GameplayStatics.GetPlayerCharacter` 0) 1.0 "VTBlend_Linear" 0.0 false)
          (`Controller.ResetIgnoreMoveInput` _returnvalue_2)
          (`Controller.ResetIgnoreLookInput` _returnvalue_2)
          (set `PlayerController.bShowMouseCursor` false _returnvalue_2)
          (`WidgetBlueprintLibrary.SetFocusToGameViewport`)
          (`MoonFloristHUD.ToggleAlpha` (`self.HUD`) false))))))

(event `Key|F`
  (params (Key :type "Key Structure"))
  ;[1 1 1] Complete Order Testing
  (:`Pressed`
    (bind _result (`/Engine/EditorBlueprintResources/StandardMacros.DecrementInt` (`self.Count`))
      (:`  `
        (bind _returnvalue (`|GetDataTableRow` "/Game/User_Interface/OrderList/OrderListTable.OrderListTable" (`self.CurrentOrder`))
          (:`then`
            (bind (_orderdiscription _keyword1 _keyword2 _keyword3 _kwcolour1 _kwcolour2 _kwcolour3) (break `/Game/User_Interface/OrderList/OrderListStructure` _returnvalue))
            (bind _out_text (`/Game/User_Interface/OrderList/OL_Lib.CompleteObjective` _orderdiscription _keyword1 _keyword2 _keyword3 _result _kwcolour1 _kwcolour2 _kwcolour3))
            (`RichTextBlock.SetText` (`/Game/User_Interface/OrderList/OrderList_Widget.DescriptionRichText` (`/Game/BP_MoonFloristHUD.OrderListUI` (`self.HUD`))) (`/Game/User_Interface/OrderList/OL_Lib.To Target Text` _out_text))))))))

(event `Key|E`
  (params (Key :type "Key Structure"))
  (bind _returnvalue (`GameplayStatics.GetPlayerController` 0))
  (bind _returnvalue_2 (`GameplayStatics.GetPlayerController` 0))
  ;[0 0 0] Interaction for Inventory
  (:`Pressed`
    (bind (_returnvalue_3 _hitactor) (`self.InteractionCheck`))
    (bind _asstorage (cast `/Game/Interactables/Storage` _hitactor))
    (if _returnvalue_3
      (`/Engine/EditorBlueprintResources/StandardMacros.FlipFlop`
        (:`A`
          (`PlayerController.SetViewTargetWithBlend` _returnvalue_2 _asstorage 1.0 "VTBlend_Linear" 0.0 false)
          (`Controller.SetIgnoreMoveInput` _returnvalue_2 true)
          (`Controller.SetIgnoreLookInput` _returnvalue_2 true)
          (bind _asstorage_window (cast `/Game/User_Interface/Storage/StorageWindow` (`WidgetComponent.GetUserWidgetObject` (`/Game/Interactables/Storage.Widget` _asstorage))))
          (for _array_element (`/Game/User_Interface/Storage/StorageWidget.StorageSlots` (`/Game/User_Interface/Storage/StorageWindow.StorageWidget_67` _asstorage_window))
            (`/Game/User_Interface/Storage/StorageSlot.UpdateSlot` _array_element)
            (`MoonFloristHUD.ToggleAlpha` (`self.HUD`) true)))
        (:`B`
          (`PlayerController.SetViewTargetWithBlend` (`GameplayStatics.GetPlayerController` 0) (`GameplayStatics.GetPlayerCharacter` 0) 1.0 "VTBlend_Linear" 0.0 false)
          (`Controller.ResetIgnoreMoveInput` _returnvalue)
          (`Controller.ResetIgnoreLookInput` _returnvalue)
          (set `PlayerController.bShowMouseCursor` false _returnvalue)
          (`WidgetBlueprintLibrary.SetFocusToGameViewport`)
          (`MoonFloristHUD.ToggleAlpha` (`self.HUD`) false)))
      (else
        (`KismetSystemLibrary.PrintString` "Not Close Enough to Access Inventory")))))

(event `Key|Tab`
  (params (Key :type "Key Structure"))
  (bind _orderlistui (`/Game/BP_MoonFloristHUD.OrderListUI` (`self.HUD`)))
  (bind _orderlistui_2 (`/Game/BP_MoonFloristHUD.OrderListUI` (`self.HUD`)))
  ;[1 1 1] Play Animation For OrderList
  (:`Pressed`
    (`/Engine/EditorBlueprintResources/StandardMacros.FlipFlop` :!label _label
      (:`A`
        (`UserWidget.PlayAnimation` _orderlistui (`/Game/User_Interface/OrderList/OrderList_Widget.PullOutAnimation` _orderlistui) 0.0 1 "Reverse" 2.0)
        (`KismetSystemLibrary.PrintString` "Back"))
      (:`B`
        (`UserWidget.PlayAnimation` _orderlistui_2 (`/Game/User_Interface/OrderList/OrderList_Widget.PullOutAnimation` _orderlistui_2) 0.0 1 "Forward" 2.0)
        (`KismetSystemLibrary.PrintString` "forward")))))

(event `Key|Z`
  (params (Key :type "Key Structure"))
  ;[1 1 1] Play Animation For OrderList
  (:`Pressed`
    (goto _label)))

(event `Key|E`
  (params (Key :type "Key Structure"))
  (bind _returnvalue (`GameplayStatics.GetPlayerController` 0))
  (bind _returnvalue_2 (`GameplayStatics.GetPlayerController` 0))
  (bind _returnvalue_3 (`GameplayStatics.GetPlayerController` 0))
  ;[0 0 0] Radio Interactiuon
  (:`Pressed`
    (bind (_returnvalue_4 _hitactor) (`self.InteractionCheck`))
    (bind _asbp_radio (cast `/Game/Interactables/BP_Radio` _hitactor))
    (if _returnvalue_4
      (set `self.RadioBtns` (`/Game/Interactables/BP_Radio.RadioBtn` _asbp_radio))
      (`/Engine/EditorBlueprintResources/StandardMacros.FlipFlop`
        (:`A`
          (`WidgetBlueprintLibrary.SetInputMode_GameAndUIEx` (`GameplayStatics.GetPlayerController` 0) (`WidgetComponent.GetUserWidgetObject` (`/Game/Interactables/BP_Radio.Widget` _asbp_radio)))
          (`SceneComponent.SetVisibility` (`self.RadioBtns`) true false)
          (`PlayerController.SetViewTargetWithBlend` _returnvalue_3 _asbp_radio 1.0 "VTBlend_Linear" 0.0 false)
          (`Controller.SetIgnoreMoveInput` _returnvalue_3 true)
          (`Controller.SetIgnoreLookInput` _returnvalue_3 true)
          (set `PlayerController.bShowMouseCursor` true (`GameplayStatics.GetPlayerController` 0))
          (`MoonFloristHUD.ToggleAlpha` (`self.HUD`) true))
        (:`B`
          (`WidgetBlueprintLibrary.SetInputMode_GameOnly` _returnvalue)
          (`PlayerController.SetViewTargetWithBlend` _returnvalue (`GameplayStatics.GetPlayerCharacter` 0) 1.0 "VTBlend_Linear" 0.0 false)
          (`Controller.ResetIgnoreMoveInput` _returnvalue_2)
          (`Controller.ResetIgnoreLookInput` _returnvalue_2)
          (set `PlayerController.bShowMouseCursor` false _returnvalue_2)
          (`WidgetBlueprintLibrary.SetFocusToGameViewport`)
          (`SceneComponent.SetVisibility` (`self.RadioBtns`) false false)
          (`MoonFloristHUD.ToggleAlpha` (`self.HUD`) false)))
      (else
        (`KismetSystemLibrary.PrintString` "Not Close Enough To access Radio")))))

(event `Key|E`
  (params (Key :type "Key Structure"))
  (bind _returnvalue (`GameplayStatics.GetPlayerController` 0))
  (bind _returnvalue_2 (`GameplayStatics.GetPlayerController` 0))
  ;[0 0 0] Interaction for Plantation
  (:`Pressed`
    (bind (_returnvalue_3 _hitactor) (`self.InteractionCheck`))
    (bind _asbp_flower_plantation (cast `/Game/Interactables/BP_FlowerPlantation` _hitactor))
    (if _returnvalue_3
      (bind _output_get (set `self.CurrentSelectedPlanter` _asbp_flower_plantation))
      (`/Engine/EditorBlueprintResources/StandardMacros.FlipFlop`
        (:`A`
          (`SceneComponent.SetVisibility` (`/Game/Interactables/BP_FlowerPlantation.Plant` (`self.CurrentSelectedPlanter`)) true false)
          (`SceneComponent.SetVisibility` (`/Game/Interactables/BP_FlowerPlantation.Widget` (`self.CurrentSelectedPlanter`)) true false)
          (`SceneComponent.SetVisibility` (`/Game/Interactables/BP_FlowerPlantation.ConfirmBtn` (`self.CurrentSelectedPlanter`)) true false)
          (`PlayerController.SetViewTargetWithBlend` _returnvalue _output_get 1.0 "VTBlend_Linear" 0.0 false)
          (`Controller.SetIgnoreMoveInput` _returnvalue true)
          (`Controller.SetIgnoreLookInput` _returnvalue true)
          (set `PlayerController.bShowMouseCursor` true (`GameplayStatics.GetPlayerController` 0))
          (`MoonFloristHUD.ToggleAlpha` (`self.HUD`) true))
        (:`B`
          (`PlayerController.SetViewTargetWithBlend` (`GameplayStatics.GetPlayerController` 0) (`GameplayStatics.GetPlayerCharacter` 0) 1.0 "VTBlend_Linear" 0.0 false)
          (`Controller.ResetIgnoreMoveInput` _returnvalue_2)
          (`Controller.ResetIgnoreLookInput` _returnvalue_2)
          (set `PlayerController.bShowMouseCursor` false _returnvalue_2)
          (`WidgetBlueprintLibrary.SetFocusToGameViewport`)
          (`SceneComponent.SetVisibility` (`/Game/Interactables/BP_FlowerPlantation.Widget` (`self.CurrentSelectedPlanter`)) false false)
          (`SceneComponent.SetVisibility` (`/Game/Interactables/BP_FlowerPlantation.ConfirmBtn` (`self.CurrentSelectedPlanter`)) false false)
          (`SceneComponent.SetVisibility` (`/Game/Interactables/BP_FlowerPlantation.Plant` (`self.CurrentSelectedPlanter`)) false false)
          (`MoonFloristHUD.ToggleAlpha` (`self.HUD`) false)))
      (else
        (`KismetSystemLibrary.PrintString` "Not Close Enough to Access Plantation")))))

(event `Lft_BTN`
  ;[1 1 1] Plant 3D widget button
  (`SceneComponent.SetVisibility` (`/Game/Interactables/BP_FlowerPlantation.Cylinder` (`self.CurrentSelectedPlanter`)) true false)
  (set `/Game/Interactables/BP_FlowerPlantation.IsHologram` true (`self.CurrentSelectedPlanter`))
  (`self.PlanterLeftBtn`)
  (bind (_direction _activate) (`Timeline|HologramActivate` :!via `PlayFromStart` :!label _label_2)
    (:`Update`
      (`KismetMaterialLibrary.SetScalarParameterValue` "/Game/HologramShader/MPC_Hologram.MPC_Hologram" "Activation" _activate))))

(event `Rgt_BTN`
  ;[1 1 1] Plant 3D widget button
  (`SceneComponent.SetVisibility` (`/Game/Interactables/BP_FlowerPlantation.Cylinder` (`self.CurrentSelectedPlanter`)) true false)
  (set `/Game/Interactables/BP_FlowerPlantation.IsHologram` true (`self.CurrentSelectedPlanter`))
  (`self.PlanterRightBtn`)
  (goto _label_2 :!via `PlayFromStart`))

(event `Plant_BTN`
  (bind _currentselectedplanter (`self.CurrentSelectedPlanter`))
  (bind _cover (`/Game/Interactables/BP_FlowerPlantation.Cover` _currentselectedplanter))
  (bind _cover_2 (`/Game/Interactables/BP_FlowerPlantation.Cover` _currentselectedplanter))
  (bind (_relativelocation_x _relativelocation_y) (`KismetMathLibrary.BreakVector` (`SceneComponent.RelativeLocation` _cover)))
  (bind (_relativelocation_x_2 _relativelocation_y_2) (`KismetMathLibrary.BreakVector` (`SceneComponent.RelativeLocation` _cover_2)))
  ;[1 1 1] Plant 3D widget button
  (set `/Game/Interactables/BP_FlowerPlantation.IsHologram` false _currentselectedplanter)
  (set `/Game/Interactables/BP_FlowerPlantation.Planted` true _currentselectedplanter)
  (`self.PlanterPlantBtn`)
  (`KismetSystemLibrary.Delay` 1.0)
  (bind (_direction _location) (`Timeline|CloseHatch` :!via `PlayFromStart`)
    (:`Update`
      (`SceneComponent.K2_SetRelativeLocation` _cover (`KismetMathLibrary.MakeVector` _relativelocation_x _relativelocation_y _location) false false))
    (:`Finished`
      (`self.PlantTimer`
        (:`Completed`
          (`self.CompleteGrowth`)
          (bind (_direction_2 _location_2) (`Timeline|OpenHatch` :!via `ReverseFromEnd`)
            (:`Update`
              (`SceneComponent.K2_SetRelativeLocation` _cover_2 (`KismetMathLibrary.MakeVector` _relativelocation_x_2 _relativelocation_y_2 _location_2) false false))
            (:`Finished`
              (set `self.CanCollect` true))))))))

(event `Collect_BTN`
  ;[1 1 1] Plant 3D widget button
  (`self.CollectPlantBtn`)
  (`KismetSystemLibrary.Delay` 2.0)
  (`self.ResetPlantation`))

(fn `CollectPlantBtn`
  (bind _itemstacks (`self.ItemStacks`))
  (bind _itemstacks_2 (`self.ItemStacks`))
  (bind _itemstacks_3 (`self.ItemStacks`))
  (bind _itemstacks_4 (`self.ItemStacks`))
  (bind _returnvalue (`KismetArrayLibrary.Array_Find` (`self.ItemsInStorage`) "NewEnumerator3"))
  (bind _returnvalue_2 (`KismetArrayLibrary.Array_Find` (`self.ItemsInStorage`) "NewEnumerator0"))
  (bind _returnvalue_3 (`KismetArrayLibrary.Array_Find` (`self.ItemsInStorage`) "NewEnumerator1"))
  (bind _returnvalue_4 (`KismetArrayLibrary.Array_Find` (`self.ItemsInStorage`) "NewEnumerator2"))
  ;[1 0 0] Red Flower
  (if (== (`self.FlowerSelected`) (`|GetArrayItem` (`/Game/Interactables/BP_FlowerPlantation.FlowerMesh` (`self.CurrentSelectedPlanter`))))
    (`KismetArrayLibrary.Array_Set` _itemstacks_2 _returnvalue_2 (+ (`|GetArrayItem` _itemstacks_2 _returnvalue_2) 1))
    (`StaticMeshComponent.SetStaticMesh` (`/Game/Interactables/BP_FlowerPlantation.Plant` (`self.CurrentSelectedPlanter`)) null :!label _label)
    (set `self.CanCollect` false)
    (return)
    (else
      ;[0 0.1291 1] Blue Flower
      (if (== (`self.FlowerSelected`) (`|GetArrayItem` (`/Game/Interactables/BP_FlowerPlantation.FlowerMesh` (`self.CurrentSelectedPlanter`)) 1))
        (`KismetArrayLibrary.Array_Set` _itemstacks_3 _returnvalue_3 (+ (`|GetArrayItem` _itemstacks_3 _returnvalue_3) 1))
        (goto _label)
        (else
          ;[1 0.8718 0] Yellow Flower
          (if (== (`self.FlowerSelected`) (`|GetArrayItem` (`/Game/Interactables/BP_FlowerPlantation.FlowerMesh` (`self.CurrentSelectedPlanter`)) 2))
            (`KismetArrayLibrary.Array_Set` _itemstacks_4 _returnvalue_4 (+ (`|GetArrayItem` _itemstacks_4 _returnvalue_4) 1))
            (goto _label)
            (else
              ;[1 1 1] White Flower
              (if (== (`self.FlowerSelected`) (`|GetArrayItem` (`/Game/Interactables/BP_FlowerPlantation.FlowerMesh` (`self.CurrentSelectedPlanter`)) 3))
                (`KismetArrayLibrary.Array_Set` _itemstacks _returnvalue (+ (`|GetArrayItem` _itemstacks _returnvalue) 1) true)
                (goto _label)
                (else
                  (`KismetSystemLibrary.PrintString` "Collect Plant not adding to inventory" true true (struct :`R` 1.0 :`B` 0.138062 :`A` 1.0) 5.0))))))))))

(fn `CompleteGrowth`
  (`StaticMeshComponent.SetStaticMesh` (`/Game/Interactables/BP_FlowerPlantation.Plant` (`self.CurrentSelectedPlanter`)) (`self.FlowerSelected`))
  (return))

(fn `InteractionCheck`
  (returns (ReturnValue :type Boolean) (HitActor :type "Actor Object Reference"))
  (bind _returnvalue (`self.RaycastCheck`))
  (bind (_bblockinghit _binitialoverlap _time _distance _location _impactpoint _normal _impactnormal _physmat _hitactor _hitcomponent _hitbonename _hititem _faceindex _tracestart) (`GameplayStatics.BreakHitResult` _returnvalue))
  (return (<= (`KismetMathLibrary.VSize` (- _tracestart (`self.K2_GetActorLocation` _hitactor))) (`self.Raycast Check Distance`)) _hitactor))

(fn `LineTraceForLookAt`
  (returns (HitActor :type "Actor Object Reference"))
  (bind _rootcomponent (`Actor.RootComponent` (`GameplayStatics.GetPlayerCharacter` 0)))
  (bind _returnvalue (`SceneComponent.K2_GetComponentLocation` _rootcomponent))
  (bind _outhit (`KismetSystemLibrary.LineTraceSingle` :`Start` (+ _returnvalue (0.0 0.0 20.0)) :`End` (+ _returnvalue (* (`KismetMathLibrary.GetForwardVector` (`SceneComponent.K2_GetComponentRotation` _rootcomponent)) (`self.RaycastDistance`))) :`TraceChannel` "TraceTypeQuery1" :`DrawDebugType` "ForOneFrame" :`DrawTime` 2.0))
  (return (`.HitActor` (`GameplayStatics.BreakHitResult` _outhit))))

(fn `LineTraceForLowObjects`
  (returns (HitActor :type "Actor Object Reference"))
  (bind _rootcomponent (`Actor.RootComponent` (`GameplayStatics.GetPlayerCharacter` 0)))
  (bind _returnvalue (`SceneComponent.K2_GetComponentLocation` _rootcomponent))
  (bind _outhit (`KismetSystemLibrary.LineTraceSingle` :`Start` (+ _returnvalue (0.0 0.0 -20.0)) :`End` (+ _returnvalue (* (`KismetMathLibrary.GetForwardVector` (`SceneComponent.K2_GetComponentRotation` _rootcomponent)) (`self.RaycastDistance`))) :`TraceChannel` "TraceTypeQuery1" :`DrawDebugType` "ForOneFrame" :`DrawTime` 2.0))
  (return (`.HitActor` (`GameplayStatics.BreakHitResult` _outhit))))

(fn `PlanterLeftBtn`
  (locals (Plant :type "StaticMeshComponent Object Reference"))
  (bind _currentselectedplanter (`self.CurrentSelectedPlanter`))
  (bind _plant (`local.Plant`))
  (bind _flowermesh (`/Game/Interactables/BP_FlowerPlantation.FlowerMesh` _currentselectedplanter))
  (`/Engine/EditorBlueprintResources/StandardMacros.DecrementInt` (`self.PlantCounter`)
    (:`  `
      (set `local.Plant` (`/Game/Interactables/BP_FlowerPlantation.Plant` _currentselectedplanter))
      (if (< (`self.PlantCounter`) 0)
        (bind _output_get (set `self.PlantCounter` 3))
        (`StaticMeshComponent.SetStaticMesh` _plant (`|GetArrayItem` _flowermesh _output_get))
        (`PrimitiveComponent.SetMaterial` _plant 0 "/Game/HologramShader/MI_MasterMeshHologram.MI_MasterMeshHologram")
        (else
          (`StaticMeshComponent.SetStaticMesh` _plant (`|GetArrayItem` _flowermesh (`self.PlantCounter`)))
          (`PrimitiveComponent.SetMaterial` _plant 0 "/Game/HologramShader/MI_MasterMeshHologram.MI_MasterMeshHologram")))
      (`KismetMaterialLibrary.SetScalarParameterValue` "/Game/HologramShader/MPC_Hologram.MPC_Hologram" "Activation" 1.0)
      (return))))

(fn `PlanterPlantBtn`
  (bind _currentselectedplanter (`self.CurrentSelectedPlanter`))
  (bind _itemstacks (`self.ItemStacks`))
  (bind _itemstacks_2 (`self.ItemStacks`))
  (bind _itemstacks_3 (`self.ItemStacks`))
  (bind _itemstacks_4 (`self.ItemStacks`))
  (bind _returnvalue (`KismetArrayLibrary.Array_Find` (`self.ItemsInStorage`) "NewEnumerator7"))
  (bind _returnvalue_2 (`KismetArrayLibrary.Array_Find` (`self.ItemsInStorage`) "NewEnumerator4"))
  (bind _returnvalue_3 (`KismetArrayLibrary.Array_Find` (`self.ItemsInStorage`) "NewEnumerator5"))
  (bind _returnvalue_4 (`KismetArrayLibrary.Array_Find` (`self.ItemsInStorage`) "NewEnumerator6"))
  (bind _plant (`/Game/Interactables/BP_FlowerPlantation.Plant` _currentselectedplanter))
  (bind _output (`|GetArrayItem` _itemstacks _returnvalue))
  (bind _output_2 (`|GetArrayItem` _itemstacks_2 _returnvalue_2))
  (bind _output_3 (`|GetArrayItem` _itemstacks_3 _returnvalue_3))
  (bind _output_4 (`|GetArrayItem` _itemstacks_4 _returnvalue_4))
  (set `self.FlowerSelected` (`StaticMeshComponent.StaticMesh` _plant))
  ;[1 0 0] Red Flower
  (if (== (`self.FlowerSelected`) (`|GetArrayItem` (`/Game/Interactables/BP_FlowerPlantation.FlowerMesh` (`self.CurrentSelectedPlanter`))))
    (if (> _output_2 0)
      (`KismetArrayLibrary.Array_Set` _itemstacks_2 _returnvalue_2 (- _output_2 1))
      (`StaticMeshComponent.SetStaticMesh` _plant "/Game/Meshes/Flowers/Sappling.Sappling" :!label _label)
      (`PrimitiveComponent.SetMaterial` _plant 0 "/Game/Materials/M_Default.M_Default")
      (`SceneComponent.SetVisibility` (`/Game/Interactables/BP_FlowerPlantation.Cylinder` _currentselectedplanter) false false)
      (return))
    (else
      ;[0 0.1291 1] Blue Flower
      (if (== (`self.FlowerSelected`) (`|GetArrayItem` (`/Game/Interactables/BP_FlowerPlantation.FlowerMesh` (`self.CurrentSelectedPlanter`)) 1))
        (if (> _output_3 0)
          (`KismetArrayLibrary.Array_Set` _itemstacks_3 _returnvalue_3 (- _output_3 1))
          (goto _label))
        (else
          ;[1 0.8718 0] Yellow Flower
          (if (== (`self.FlowerSelected`) (`|GetArrayItem` (`/Game/Interactables/BP_FlowerPlantation.FlowerMesh` (`self.CurrentSelectedPlanter`)) 2))
            (if (> _output_4 0)
              (`KismetArrayLibrary.Array_Set` _itemstacks_4 _returnvalue_4 (- _output_4 1))
              (goto _label))
            (else
              ;[1 1 1] White Flower
              (if (== (`self.FlowerSelected`) (`|GetArrayItem` (`/Game/Interactables/BP_FlowerPlantation.FlowerMesh` (`self.CurrentSelectedPlanter`)) 3))
                (if (> _output 0)
                  (`KismetArrayLibrary.Array_Set` _itemstacks _returnvalue (- _output 1) true)
                  (goto _label))
                (else
                  (`KismetSystemLibrary.PrintString` "Collect Plant not adding to inventory" true true (struct :`R` 1.0 :`B` 0.138062 :`A` 1.0) 5.0))))))))))

(fn `PlanterRightBtn`
  (locals (PlantRight :type "StaticMeshComponent Object Reference"))
  (bind _currentselectedplanter (`self.CurrentSelectedPlanter`))
  (bind _plantright (`local.PlantRight`))
  (bind _flowermesh (`/Game/Interactables/BP_FlowerPlantation.FlowerMesh` _currentselectedplanter))
  (`/Engine/EditorBlueprintResources/StandardMacros.IncrementInt` (`self.PlantCounter`)
    (:`  `
      (set `local.PlantRight` (`/Game/Interactables/BP_FlowerPlantation.Plant` _currentselectedplanter))
      (if (> (`self.PlantCounter`) 3)
        (bind _output_get (set `self.PlantCounter` 0))
        (`StaticMeshComponent.SetStaticMesh` _plantright (`|GetArrayItem` _flowermesh _output_get))
        (`PrimitiveComponent.SetMaterial` _plantright 0 "/Game/HologramShader/MI_MasterMeshHologram.MI_MasterMeshHologram")
        (else
          (`StaticMeshComponent.SetStaticMesh` _plantright (`|GetArrayItem` _flowermesh (`self.PlantCounter`)))
          (`PrimitiveComponent.SetMaterial` _plantright 0 "/Game/HologramShader/MI_MasterMeshHologram.MI_MasterMeshHologram")))
      (`KismetMaterialLibrary.SetScalarParameterValue` "/Game/HologramShader/MPC_Hologram.MPC_Hologram" "Activation" 1.0)
      (return))))

(fn `ResetPlantation`
  (bind _currentselectedplanter (`self.CurrentSelectedPlanter`))
  (`SceneComponent.SetVisibility` (`/Game/Interactables/BP_FlowerPlantation.Cylinder` _currentselectedplanter) true false)
  (set `/Game/Interactables/BP_FlowerPlantation.IsHologram` true _currentselectedplanter)
  (set `/Game/Interactables/BP_FlowerPlantation.Planted` false _currentselectedplanter)
  (`self.Lft_BTN`)
  (return))

(fn `UserConstructionScript`)