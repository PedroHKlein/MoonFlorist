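; BP_Radio is an interactable radio that plays music on BeginPlay and shows track and volume info on a widget component.
; LeftBtn and RightBtn step forward and back through wrapping song arrays, updating title, artist and album cover.
; Each switch briefly sets a static cue, then fades in the new track at a random offset to mimic tuning.
; Volume events step the audio multiplier and refresh the percentage readout.
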(event `self.ReceiveBeginPlay`
  (bind _radiosource (`self.RadioSource`))
  (`self.EnableInput` (`GameplayStatics.GetPlayerController` 0))
  (`AudioComponent.SetSound` _radiosource (`self.Sound`))
  (`AudioComponent.Play` _radiosource 0.0)
  (`AudioComponent.FadeIn` (`self.RadioSource`) 10.0 1.0 0.0)
  (bind _returnvalue (`|CreateWidget` "/Game/Radio/RadioWidget.RadioWidget_C"))
  (bind _output_get (set `self.WidgetReference` _returnvalue))
  (`WidgetComponent.SetWidget` (`self.Widget`) _output_get)
  (`AudioComponent.SetVolumeMultiplier` (`self.RadioSource`) 0.5)
  (`SceneComponent.SetVisibility` (`self.RadioBtn`) false false)
  (`self.StartingVolume`)
  (`self.GetInteractableName`))

(event `LeftBtn`
  (bind _returnvalue (`KismetMathLibrary.RandomFloatInRange` 20.0 100.0))
  (bind _radiosource (`self.RadioSource`))
  (bind _radiosource_2 (`self.RadioSource`))
  (if (== (`self.Song`) (`self.MaxSong`))
    (set `self.Song` 0)
    (else
      (set `self.Song` (+ (`self.Song`) 1))))
  (bind _asradio_widget (cast `/Game/Radio/RadioWidget` (`self.WidgetReference`) :!label _label))
  (`TextBlock.SetText` (`/Game/Radio/RadioWidget.Title` _asradio_widget) (`|GetArrayItem` (`self.Titles`) (`self.Song`)))
  (`TextBlock.SetText` (`/Game/Radio/RadioWidget.Autor` _asradio_widget) (`|GetArrayItem` (`self.Autors`) (`self.Song`)))
  (`Image.SetBrushFromTexture` (`/Game/Radio/RadioWidget.AlbumCOver` _asradio_widget) (`|GetArrayItem` (`self.AlbumCovers`) (`self.Song`)) false)
  (set `self.Sound` (`|GetArrayItem` (`self.Sounds`) (`self.Song`)))
  (`AudioComponent.SetSound` _radiosource_2 "/Game/Radio/Radio_Static_Cue.Radio_Static_Cue")
  (`KismetSystemLibrary.Delay` (`KismetMathLibrary.RandomFloatInRange` 0.1 0.3))
  (`AudioComponent.Play` _radiosource_2 (`KismetMathLibrary.RandomFloatInRange` 20.0 100.0))
  (`AudioComponent.FadeOut` _radiosource 10.0 0.0)
  (`AudioComponent.SetSound` _radiosource (`self.Sound`))
  (`AudioComponent.Play` _radiosource _returnvalue)
  (`AudioComponent.FadeIn` (`self.RadioSource`) 10.0 1.0 _returnvalue)
  (`KismetSystemLibrary.PrintString` (`KismetSystemLibrary.GetDisplayName` (`self.Sound`))))

(event `RightBtn`
  (if (== (`self.Song`) 0)
    (set `self.Song` (`self.MaxSong`))
    (goto _label)
    (else
      (set `self.Song` (- (`self.Song`) 1))
      (goto _label))))

(event `VolumeUP`
  (bind _volume (`self.Volume`))
  (if (< (`self.Volume`) 1.0)
    (set `self.Volume` (+ (`self.Volume`) 0.1))
    (`AudioComponent.SetVolumeMultiplier` (`self.RadioSource`) _volume :!label _label_2)
    (`KismetSystemLibrary.PrintString` (`KismetStringLibrary.Conv_DoubleToString` _volume))
    (`TextBlock.SetText` (`/Game/Radio/RadioWidget.Volume` (`self.WidgetReference`)) (`KismetTextLibrary.Conv_StringToText` (`KismetStringLibrary.Concat_StrStr` (`KismetStringLibrary.Conv_IntToString` (`KismetMathLibrary.FTrunc` (* _volume 100.0))) "%")))))

(event `VolumeDOWN`
  (if (> (`self.Volume`) 0.1)
    (set `self.Volume` (- (`self.Volume`) 0.1))
    (goto _label_2)
    (else
      (set `self.Volume` 0.0)
      (goto _label_2))))

(fn `StartingVolume`
  (bind _output_get (set `self.Volume` 0.4))
  (`AudioComponent.SetVolumeMultiplier` (`self.RadioSource`) _output_get)
  (`TextBlock.SetText` (`/Game/Radio/RadioWidget.Volume` (`self.WidgetReference`)) (`KismetTextLibrary.Conv_StringToText` (`KismetStringLibrary.Concat_StrStr` (`KismetStringLibrary.Conv_IntToString` (`KismetMathLibrary.FTrunc` (* (`self.Volume`) 100.0))) "%"))))

(fn `UserConstructionScript`)