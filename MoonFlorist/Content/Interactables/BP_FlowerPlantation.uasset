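; Interactable flower plantation actor that displays its plant as a rotating hologram, with no planting logic in these graphs.
; The construction script applies the flower mesh and hologram material, then switches on the hologram material parameter collection.
; BeginPlay hides the confirm widget and caches the first Moon Florist character as the player.
; Tick spins the plant while it is a hologram and toggles floating text using a distance threshold.
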(event `self.ReceiveBeginPlay`
  (`KismetMaterialLibrary.CreateDynamicMaterialInstance` "/Game/HologramShader/MI_MasterHologram.MI_MasterHologram")
  (`KismetMaterialLibrary.CreateDynamicMaterialInstance` "/Game/HologramShader/MI_MasterMeshHologram.MI_MasterMeshHologram")
  (`self.GetInteractableName`)
  (`SceneComponent.SetVisibility` (`self.Widget`) false false)
  (`SceneComponent.SetVisibility` (`self.ConfirmBtn`) false false)
  (bind _outactors (`GameplayStatics.GetAllActorsOfClass` "/Game/BP_MoonFloristCharacter.BP_MoonFloristCharacter_C"))
  (set `self.Player` (`|GetArrayItem` _outactors)))

(event `self.ReceiveTick`
  (params (DeltaSeconds :type "Float (single-precision)"))
  (if (`self.IsHologram`)
    (`SceneComponent.K2_AddLocalRotation` (`self.Plant`) (* (`self.Rotation Axis`) (`self.Rotation Speed`)) false false))
  (`self.ToggleVisiblity-FloatingText(Actor)` 300.0))

(fn `UserConstructionScript`
  (bind _plant (`self.Plant`))
  (`SceneComponent.SetVisibility` _plant true false)
  (`SceneComponent.SetVisibility` (`self.Cylinder`) true false)
  (set `self.IsHologram` true)
  (`StaticMeshComponent.SetStaticMesh` _plant "/Game/Meshes/Flowers/Flower2_low.Flower2_low")
  (`PrimitiveComponent.SetMaterial` _plant 0 "/Game/HologramShader/MI_MasterMeshHologram.MI_MasterMeshHologram")
  (`KismetMaterialLibrary.SetScalarParameterValue` "/Game/HologramShader/MPC_Hologram.MPC_Hologram" "Activation" 1.0))