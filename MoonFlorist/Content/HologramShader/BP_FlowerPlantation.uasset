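; Flower plantation actor that displays one of four selectable flower meshes as a rotating hologram.
; Keys 1 to 4 swap the Plant mesh, apply the hologram material and restart the TurnHologramON timeline, which animates Activation in MPC_Hologram.
; Tick spins the Plant by RotationAxis times RotationSpeed, without delta-time scaling.
; The construction script creates two dynamic material instances but never stores or applies them.
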(event `self.ReceiveBeginPlay`
  (`self.EnableInput` (`GameplayStatics.GetPlayerController` 0)))

(event `Key|One`
  (params (Key :type "Key Structure"))
  (bind _plant (`self.Plant`))
  (:`Pressed`
    (`StaticMeshComponent.SetStaticMesh` _plant "/Game/Meshes/Flowers/Flower1_low.Flower1_low")
    (`PrimitiveComponent.SetMaterial` _plant 0 "/Game/HologramShader/MI_MasterMeshHologram.MI_MasterMeshHologram")
    (`KismetMaterialLibrary.SetScalarParameterValue` "/Game/HologramShader/MPC_Hologram.MPC_Hologram" "Activation" 1.0 :!label _label)
    (bind (_direction _activate) (`Timeline|TurnHologramON` :!via `PlayFromStart`)
      (:`Update`
        (`KismetMaterialLibrary.SetScalarParameterValue` "/Game/HologramShader/MPC_Hologram.MPC_Hologram" "Activation" _activate)))))

(event `Key|Two`
  (params (Key :type "Key Structure"))
  (bind _plant (`self.Plant`))
  (:`Pressed`
    (`StaticMeshComponent.SetStaticMesh` _plant "/Game/Meshes/Flowers/Flower2_low.Flower2_low")
    (`PrimitiveComponent.SetMaterial` _plant 0 "/Game/HologramShader/MI_MasterMeshHologram.MI_MasterMeshHologram")
    (goto _label)))

(event `Key|Three`
  (params (Key :type "Key Structure"))
  (bind _plant (`self.Plant`))
  (:`Pressed`
    (`StaticMeshComponent.SetStaticMesh` _plant "/Game/Meshes/Flowers/Flower3_low.Flower3_low")
    (`PrimitiveComponent.SetMaterial` _plant 0 "/Game/HologramShader/MI_MasterMeshHologram.MI_MasterMeshHologram")
    (goto _label)))

(event `Key|Four`
  (params (Key :type "Key Structure"))
  (bind _plant (`self.Plant`))
  (:`Pressed`
    (`StaticMeshComponent.SetStaticMesh` _plant "/Game/Meshes/Flowers/Flower4_low.Flower4_low")
    (`PrimitiveComponent.SetMaterial` _plant 0 "/Game/HologramShader/MI_MasterMeshHologram.MI_MasterMeshHologram")
    (goto _label)))

(event `self.ReceiveTick`
  (params (DeltaSeconds :type "Float (single-precision)"))
  (`SceneComponent.K2_AddLocalRotation` (`self.Plant`) (* (`self.Rotation Axis`) (`self.Rotation Speed`)) false false))

(fn `UserConstructionScript`
  (`KismetMaterialLibrary.CreateDynamicMaterialInstance` "/Game/HologramShader/MI_MasterHologram.MI_MasterHologram")
  (`KismetMaterialLibrary.CreateDynamicMaterialInstance` "/Game/HologramShader/MI_MasterMeshHologram.MI_MasterMeshHologram"))