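; Space skybox actor that applies a chosen sky material to its static mesh and controls the look of the sky.
; It writes star brightness, scene brightness, power, sky rotation and rotation axis from its variables into the MP_SpaceSkybox material parameter collection.
; The construction script and BeginPlay run the same setup, so edits show in the editor and are reapplied when play starts.
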(event `self.ReceiveBeginPlay`
  (`PrimitiveComponent.SetMaterial` (`self.StaticMesh`) 0 (`self.Material`))
  (`KismetMaterialLibrary.SetScalarParameterValue` "/Game/Skybox/MP_SpaceSkybox.MP_SpaceSkybox" "Start Brightness" (`self.Star Brightness`))
  (`KismetMaterialLibrary.SetScalarParameterValue` "/Game/Skybox/MP_SpaceSkybox.MP_SpaceSkybox" "Scene Brightness" (`self.Scene Brightness`))
  (`KismetMaterialLibrary.SetScalarParameterValue` "/Game/Skybox/MP_SpaceSkybox.MP_SpaceSkybox" "Power" (`self.Power`))
  (`KismetMaterialLibrary.SetScalarParameterValue` "/Game/Skybox/MP_SpaceSkybox.MP_SpaceSkybox" "SkyRotation" (`self.SkyRotation`))
  (`KismetMaterialLibrary.SetVectorParameterValue` "/Game/Skybox/MP_SpaceSkybox.MP_SpaceSkybox" "Axis" (`self.Axis`)))

(fn `UserConstructionScript`
  (`PrimitiveComponent.SetMaterial` (`self.StaticMesh`) 0 (`self.Material`))
  (`KismetMaterialLibrary.SetScalarParameterValue` "/Game/Skybox/MP_SpaceSkybox.MP_SpaceSkybox" "Start Brightness" (`self.Star Brightness`))
  (`KismetMaterialLibrary.SetScalarParameterValue` "/Game/Skybox/MP_SpaceSkybox.MP_SpaceSkybox" "Scene Brightness" (`self.Scene Brightness`))
  (`KismetMaterialLibrary.SetScalarParameterValue` "/Game/Skybox/MP_SpaceSkybox.MP_SpaceSkybox" "Power" (`self.Power`))
  (`KismetMaterialLibrary.SetScalarParameterValue` "/Game/Skybox/MP_SpaceSkybox.MP_SpaceSkybox" "SkyRotation" (`self.SkyRotation`))
  (`KismetMaterialLibrary.SetVectorParameterValue` "/Game/Skybox/MP_SpaceSkybox.MP_SpaceSkybox" "Axis" (`self.Axis`)))