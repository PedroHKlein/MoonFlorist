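; Player character for Moon Florist, handling look input, a sliding tablet UI and interaction with planting areas, planters and radios.
; Clicking while interacting traces under the cursor to spawn, bloom or collect BP_FlowerBloom flowers, updating seed and flower stacks in PlayerStorage.
; Planter button functions cycle hologram flower previews, then plant and collect through separate ItemStacks arrays.
; Tick lerps the tablet between two points, and opening it locks movement and look.
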(event `self.ReceiveBeginPlay`
  ;[1 1 1] Event Begin
  (bind _asbp_moon_florist_hud (cast `/Game/BP_MoonFloristHUD` (`PlayerController.GetHUD` (`GameplayStatics.GetPlayerController` 0))))
  (set `self.HUD` _asbp_moon_florist_hud)
  (set `self.HasOrder` false)
  (bind _asbp_moon_florist_character (cast `/Game/BP_MoonFloristCharacter` (`Controller.K2_GetPawn` (`GameplayStatics.GetPlayerController` 0))))
  (set `/Game/BP_MoonFloristCharacter.Player` _asbp_moon_florist_character _asbp_moon_florist_character)
  (bind _outactors (`GameplayStatics.GetAllActorsOfClass` "/Script/MoonFlorist.MyGameManager"))
  (bind _returnvalue (`MyGameManager.GetMoney` (`|GetArrayItem` _outactors)))
  (bind _output_get (set `self.CosmoCoins` _returnvalue))
  (`KismetSystemLibrary.PrintString` (`KismetStringLibrary.Conv_IntToString` _output_get))
  ;;[0 0 0] Set Tablet to Hidden At the Start
  (`SceneComponent.SetHiddenInGame` (`self.TabletUI1`) true false))

(event `InputAxis|Turn`
  (params (AxisValue :type "Float (single-precision)"))
  ;[1 1 1] Mouse Sensitivity
  (`self.AddControllerYawInput` (* AxisValue (`self.MouseSensitivity`) (`GameplayStatics.GetWorldDeltaSeconds`))))

(event `InputAxis|LookUp`
  (params (AxisValue :type "Float (single-precision)"))
  ;[1 1 1] Mouse Sensitivity
  (`self.AddControllerPitchInput` (* AxisValue (`self.MouseSensitivity`) (`GameplayStatics.GetWorldDeltaSeconds`))))

(event `InputAction|ViewTablet`
  (params (Key :type "Key Structure"))
  (bind _returnvalue (`GameplayStatics.GetPlayerController` 0))
  ;[1 1 1] Play Animation For Tablet
  (:`Pressed`
    (if (`self.Interacting`)
      (bind _asplanting_area_bp (cast `/Game/Interactables/PlantingArea_BP` (`self.CurrentInteractActor`)))
      (bind _returnvalue_2 (`WidgetComponent.GetUserWidgetObject` (`ManualPlantingArea.WidgetComp` _asplanting_area_bp)))
      (if (`Widget.IsVisible` _returnvalue_2)
        (`Widget.SetVisibility` _returnvalue_2 "Hidden")
        (else
          (`Widget.SetVisibility` _returnvalue_2 "Visible")))
      (else
        (`/Engine/EditorBlueprintResources/StandardMacros.FlipFlop`
          (:`A`
            (`Controller.SetIgnoreMoveInput` _returnvalue true)
            (`Controller.SetIgnoreLookInput` _returnvalue true)
            (set `PlayerController.bShowMouseCursor` true _returnvalue)
            (set `self.OpenTablet` true)
            (`SceneComponent.SetHiddenInGame` (`self.TabletUI1`) false false))
          (:`B`
            (`Controller.SetIgnoreMoveInput` _returnvalue false)
            (`Controller.SetIgnoreLookInput` _returnvalue false)
            (set `PlayerController.bShowMouseCursor` false _returnvalue)
            (set `self.OpenTablet` false)
            (`KismetSystemLibrary.Delay` 2.0)
            (`SceneComponent.SetHiddenInGame` (`self.TabletUI1`) true false)))))))

(event `InputAction|Action`
  (params (Key :type "Key Structure"))
  (bind _returnvalue (`GameplayStatics.GetPlayerController` 0))
  (bind _returnvalue_2 (`GameplayStatics.GetPlayerController` 0))
  (bind _currentselectedplanter (`self.CurrentSelectedPlanter`))
  (bind _currentselectedplanter_2 (`self.CurrentSelectedPlanter`))
  ;[1 1 1] Interacting
  (:`Pressed`
    (`self.DetectInteraction`)
    (bind _asplanting_area_bp (cast `/Game/Interactables/PlantingArea_BP` (`self.CurrentInteractActor`))
      (:`then`
        (if (`self.Interacting`)
          (`self.EnableInput` _asplanting_area_bp _returnvalue)
          (else
            (`self.DisableInput` _asplanting_area_bp _returnvalue))))
      (:`CastFailed`
        _))
    (bind (_returnvalue_3 _hitactor) (`self.PlantANDRadio`))
    (if _returnvalue_3
      (bind _asbp_radio (cast `/Game/Interactables/BP_Radio` _hitactor)
        (:`then`
          (`/Engine/EditorBlueprintResources/StandardMacros.FlipFlop`
            (:`A`
              (bind _radiobtn (`/Game/Interactables/BP_Radio.RadioBtn` _asbp_radio))
              (`SceneComponent.SetVisibility` _radiobtn true false))
            (:`B`
              (`SceneComponent.SetVisibility` _radiobtn false false))))
        (:`CastFailed`
          (bind _asbp_flower_plantation (cast `/Game/Interactables/BP_FlowerPlantation` _hitactor))
          (set `self.CurrentSelectedPlanter` _asbp_flower_plantation)
          (`/Engine/EditorBlueprintResources/StandardMacros.FlipFlop`
            (:`A`
              (`SceneComponent.SetVisibility` (`/Game/Interactables/BP_FlowerPlantation.Widget` _currentselectedplanter_2) true false)
              (`SceneComponent.SetVisibility` (`/Game/Interactables/BP_FlowerPlantation.ConfirmBtn` _currentselectedplanter_2) true false)
              (`self.EnableInput` _currentselectedplanter _returnvalue_2))
            (:`B`
              (`SceneComponent.SetVisibility` (`/Game/Interactables/BP_FlowerPlantation.ConfirmBtn` _currentselectedplanter_2) false false)
              (`SceneComponent.SetVisibility` (`/Game/Interactables/BP_FlowerPlantation.Widget` _currentselectedplanter_2) false false)
              (`self.DisableInput` _currentselectedplanter _returnvalue_2))))))))

(event `self.ReceiveTick`
  (params (DeltaSeconds :type "Float (single-precision)"))
  ;[1 1 1] Event Tick
  (`self.Tablet` DeltaSeconds DeltaSeconds))

(event `InputAction|Click`
  (params (Key :type "Key Structure"))
  (bind (_hitresult _returnvalue) (`PlayerController.GetHitResultUnderCursorByChannel` (`GameplayStatics.GetPlayerController` 0) "TraceTypeQuery1" true))
  (bind _playerstorage (`MoonFloristCharacter.PlayerStorage` (`self.Player`)))
  (bind _playerstorage_2 (`MoonFloristCharacter.PlayerStorage` (`self.Player`)))
  (bind (_bblockinghit _binitialoverlap _time _distance _location _impactpoint _normal _impactnormal _physmat _hitactor) (`GameplayStatics.BreakHitResult` _hitresult))
  ;[1 1 1] Checking Under Cursor
  (:`Pressed`
    (if (and (`KismetSystemLibrary.IsValid` (`self.CurrentInteractActor`)) (`self.Interacting`))
      (`KismetSystemLibrary.PrintString` "Planting")
      (if _returnvalue
        (`KismetSystemLibrary.PrintString` (`KismetSystemLibrary.GetObjectName` _hitactor))
        (bind _asplanting_area_bp (cast `/Game/Interactables/PlantingArea_BP` _hitactor)
          (:`then`
            ;[1 1 1] Planting
            (if (`|EnumInequality` (`self.ChosenFlower`) "NewEnumerator8")
              (bind _returnvalue_2 (`|SpawnActorFromClass` "/Game/Flowers/BP_FlowerBloom.BP_FlowerBloom_C" (`KismetMathLibrary.MakeTransform` _location) "Undefined" "OverrideRootScale" null null))
              (bind _output_get (set `self.GrownFlower` _returnvalue_2))
              (bind _output_get_2 (set `/Game/Flowers/BP_FlowerBloom.CurrentFlowerChosen` (`self.ChosenFlower`) _output_get))
              (bind (_returnvalue_roll _returnvalue_pitch) (`KismetMathLibrary.BreakRotator` (`self.K2_GetActorRotation` _returnvalue_2)))
              (bind (_returnvalue_roll_2 _returnvalue_pitch_2 _returnvalue_yaw) (`KismetMathLibrary.BreakRotator` (`KismetMathLibrary.FindLookAtRotation` (`self.K2_GetActorLocation` _returnvalue_2) (`SceneComponent.K2_GetComponentLocation` (`ManualPlantingArea.Camera` _asplanting_area_bp)))))
              (`self.K2_SetActorRotation` _output_get (`KismetMathLibrary.MakeRotator` _returnvalue_roll _returnvalue_pitch _returnvalue_yaw) false)
              (switch `/Game/User_Interface/Storage/ItemsList_Enum` _output_get_2
                (:`NewEnumerator0`
                  (set `self.UsedSeed` "NewEnumerator4"))
                (:`NewEnumerator1`
                  (set `self.UsedSeed` "NewEnumerator5"))
                (:`NewEnumerator2`
                  (set `self.UsedSeed` "NewEnumerator6"))
                (:`NewEnumerator3`
                  (set `self.UsedSeed` "NewEnumerator7")))
              (for _array_element (`Storage.StorageArray` _playerstorage_2)
                (bind _returnvalue_3 (`Item.GetName` _array_element))
                (if (== _returnvalue_3 (`KismetStringLibrary.Conv_StringToName` (`|GetEnumeratorNameAsString` (`self.UsedSeed`))))
                  (`Storage.DecreaseStacks` _playerstorage_2 1 _array_element)))))
          (:`CastFailed`
            ;[1 1 1] Blooming
            (bind _asbp_flower_bloom (cast `/Game/Flowers/BP_FlowerBloom` _hitactor))
            (bind _readytocollect (`/Game/Flowers/BP_FlowerBloom.ReadyToCollect` _asbp_flower_bloom))
            (if (and (== _readytocollect false) (`/Game/Flowers/BP_FlowerBloom.ReadyToBloom` _asbp_flower_bloom))
              (`SkeletalMeshComponent.PlayAnimation` (`/Game/Flowers/BP_FlowerBloom.Flower_grow_anim` _asbp_flower_bloom) "/Game/Flowers/Flower_bloom_anim.Flower_bloom_anim" false)
              (set `/Game/Flowers/BP_FlowerBloom.ReadyToCollect` true _asbp_flower_bloom)
              (`SceneComponent.SetVisibility` (`/Game/Flowers/BP_FlowerBloom.Flower_grow_anim` _asbp_flower_bloom) false false)
              (`SceneComponent.SetVisibility` (`/Game/Flowers/BP_FlowerBloom.StaticMesh` _asbp_flower_bloom) true false)
              (else
                ;[1 1 1] Collection Temp
                (if _readytocollect
                  (for _array_element_2 (`Storage.StorageArray` _playerstorage)
                    (bind _returnvalue_4 (`Item.GetName` _array_element_2))
                    (if (== _returnvalue_4 (`KismetStringLibrary.Conv_StringToName` (`|GetEnumeratorNameAsString` (`/Game/Flowers/BP_FlowerBloom.CurrentFlowerChosen` _asbp_flower_bloom))))
                      (`Storage.IncreaseStacks` _playerstorage 1 _array_element_2)))
                  (`self.K2_DestroyActor` _asbp_flower_bloom)))))))
      (else
        (`KismetSystemLibrary.PrintString` "No actor")))))

(event `Key|J`
  (params (Key :type "Key Structure"))
  (bind _playerstorage (`self.PlayerStorage`))
  ;[1 1 1] Tester Function
  (:`Pressed`
    (`Storage.IncreaseStacks` _playerstorage 5 (`|GetArrayItem` (`Storage.StorageArray` _playerstorage)))))

(fn `CollectPlantBtn`
  (bind _itemstacks (`self.ItemStacks`))
  (bind _itemstacks_2 (`self.ItemStacks`))
  (bind _itemstacks_3 (`self.ItemStacks`))
  (bind _itemstacks_4 (`self.ItemStacks`))
  (bind _returnvalue (`KismetArrayLibrary.Array_Find` (`self.ItemsInStorage`) "NewEnumerator3"))
  (bind _returnvalue_2 (`KismetArrayLibrary.Array_Find` (`self.ItemsInStorage`) "NewEnumerator0"))
  (bind _returnvalue_3 (`KismetArrayLibrary.Array_Find` (`self.ItemsInStorage`) "NewEnumerator1"))
  (bind _returnvalue_4 (`KismetArrayLibrary.Array_Find` (`self.ItemsInStorage`) "NewEnumerator2"))
  ;[1 0 0] Red Flower
  (if (== (`self.FlowerSelected`) (`|GetArrayItem` (`/Game/Interactables/BP_FlowerPlantation.FlowerMesh` (`self.CurrentSelectedPlanter`))))
    (`KismetArrayLibrary.Array_Set` _itemstacks_2 _returnvalue_2 (+ (`|GetArrayItem` _itemstacks_2 _returnvalue_2) 1))
    (`StaticMeshComponent.SetStaticMesh` (`/Game/Interactables/BP_FlowerPlantation.Plant` (`self.CurrentSelectedPlanter`)) null :!label _label)
    (set `self.CanCollect` false)
    (return)
    (else
      ;[0 0.1291 1] Blue Flower
      (if (== (`self.FlowerSelected`) (`|GetArrayItem` (`/Game/Interactables/BP_FlowerPlantation.FlowerMesh` (`self.CurrentSelectedPlanter`)) 1))
        (`KismetArrayLibrary.Array_Set` _itemstacks_3 _returnvalue_3 (+ (`|GetArrayItem` _itemstacks_3 _returnvalue_3) 1))
        (goto _label)
        (else
          ;[1 0.8718 0] Yellow Flower
          (if (== (`self.FlowerSelected`) (`|GetArrayItem` (`/Game/Interactables/BP_FlowerPlantation.FlowerMesh` (`self.CurrentSelectedPlanter`)) 2))
            (`KismetArrayLibrary.Array_Set` _itemstacks_4 _returnvalue_4 (+ (`|GetArrayItem` _itemstacks_4 _returnvalue_4) 1))
            (goto _label)
            (else
              ;[1 1 1] White Flower
              (if (== (`self.FlowerSelected`) (`|GetArrayItem` (`/Game/Interactables/BP_FlowerPlantation.FlowerMesh` (`self.CurrentSelectedPlanter`)) 3))
                (`KismetArrayLibrary.Array_Set` _itemstacks _returnvalue (+ (`|GetArrayItem` _itemstacks _returnvalue) 1) true)
                (goto _label)
                (else
                  (`KismetSystemLibrary.PrintString` "Collect Plant not adding to inventory" true true (struct :`R` 1.0 :`B` 0.138062 :`A` 1.0) 5.0))))))))))

(fn `CompleteGrowth`
  (`StaticMeshComponent.SetStaticMesh` (`/Game/Interactables/BP_FlowerPlantation.Plant` (`self.CurrentSelectedPlanter`)) (`self.FlowerSelected`))
  (return))

(fn `PlantANDRadio`
  (returns (ReturnValue :type Boolean) (HitActor :type "Actor Object Reference"))
  (bind (_bblockinghit _binitialoverlap _time _distance _location _impactpoint _normal _impactnormal _physmat _hitactor _hitcomponent _hitbonename _hititem _faceindex _tracestart) (`GameplayStatics.BreakHitResult` (`self.m_Hitsdata`)))
  (`/Engine/EditorBlueprintResources/StandardMacros.IsValid` _hitactor
    (:`Is Valid`
      (return (<= (`KismetMathLibrary.VSize` (- _tracestart (`self.K2_GetActorLocation` _hitactor))) 300.0) _hitactor))))

(fn `PlanterLeftBtn`
  (locals (Plant :type "StaticMeshComponent Object Reference"))
  (bind _currentselectedplanter (`self.CurrentSelectedPlanter`))
  (bind _plant (`local.Plant`))
  (bind _flowermesh (`/Game/Interactables/BP_FlowerPlantation.FlowerMesh` _currentselectedplanter))
  (`/Engine/EditorBlueprintResources/StandardMacros.DecrementInt` (`self.PlantCounter`)
    (:`  `
      (set `local.Plant` (`/Game/Interactables/BP_FlowerPlantation.Plant` _currentselectedplanter))
      (if (< (`self.PlantCounter`) 0)
        (bind _output_get (set `self.PlantCounter` 3))
        (`StaticMeshComponent.SetStaticMesh` _plant (`|GetArrayItem` _flowermesh _output_get))
        (`PrimitiveComponent.SetMaterial` _plant 0 "/Game/HologramShader/MI_MasterMeshHologram.MI_MasterMeshHologram")
        (else
          (`StaticMeshComponent.SetStaticMesh` _plant (`|GetArrayItem` _flowermesh (`self.PlantCounter`)))
          (`PrimitiveComponent.SetMaterial` _plant 0 "/Game/HologramShader/MI_MasterMeshHologram.MI_MasterMeshHologram")))
      (`KismetMaterialLibrary.SetScalarParameterValue` "/Game/HologramShader/MPC_Hologram.MPC_Hologram" "Activation" 1.0)
      (return))))

(fn `PlanterPlantBtn`
  (bind _currentselectedplanter (`self.CurrentSelectedPlanter`))
  (bind _itemstacks (`self.ItemStacks`))
  (bind _itemstacks_2 (`self.ItemStacks`))
  (bind _itemstacks_3 (`self.ItemStacks`))
  (bind _itemstacks_4 (`self.ItemStacks`))
  (bind _returnvalue (`KismetArrayLibrary.Array_Find` (`self.ItemsInStorage`) "NewEnumerator7"))
  (bind _returnvalue_2 (`KismetArrayLibrary.Array_Find` (`self.ItemsInStorage`) "NewEnumerator4"))
  (bind _returnvalue_3 (`KismetArrayLibrary.Array_Find` (`self.ItemsInStorage`) "NewEnumerator5"))
  (bind _returnvalue_4 (`KismetArrayLibrary.Array_Find` (`self.ItemsInStorage`) "NewEnumerator6"))
  (bind _plant (`/Game/Interactables/BP_FlowerPlantation.Plant` _currentselectedplanter))
  (bind _output (`|GetArrayItem` _itemstacks _returnvalue))
  (bind _output_2 (`|GetArrayItem` _itemstacks_2 _returnvalue_2))
  (bind _output_3 (`|GetArrayItem` _itemstacks_3 _returnvalue_3))
  (bind _output_4 (`|GetArrayItem` _itemstacks_4 _returnvalue_4))
  (set `self.FlowerSelected` (`StaticMeshComponent.StaticMesh` _plant))
  ;[1 0 0] Red Flower
  (if (== (`self.FlowerSelected`) (`|GetArrayItem` (`/Game/Interactables/BP_FlowerPlantation.FlowerMesh` (`self.CurrentSelectedPlanter`))))
    (if (> _output_2 0)
      (`KismetArrayLibrary.Array_Set` _itemstacks_2 _returnvalue_2 (- _output_2 1))
      (`StaticMeshComponent.SetStaticMesh` _plant null :!label _label)
      (`PrimitiveComponent.SetMaterial` _plant 0 "/Game/Materials/M_MasterDefault.M_MasterDefault")
      (`SceneComponent.SetVisibility` (`/Game/Interactables/BP_FlowerPlantation.Cylinder` _currentselectedplanter) false false)
      (return))
    (else
      ;[0 0.1291 1] Blue Flower
      (if (== (`self.FlowerSelected`) (`|GetArrayItem` (`/Game/Interactables/BP_FlowerPlantation.FlowerMesh` (`self.CurrentSelectedPlanter`)) 1))
        (if (> _output_3 0)
          (`KismetArrayLibrary.Array_Set` _itemstacks_3 _returnvalue_3 (- _output_3 1))
          (goto _label))
        (else
          ;[1 0.8718 0] Yellow Flower
          (if (== (`self.FlowerSelected`) (`|GetArrayItem` (`/Game/Interactables/BP_FlowerPlantation.FlowerMesh` (`self.CurrentSelectedPlanter`)) 2))
            (if (> _output_4 0)
              (`KismetArrayLibrary.Array_Set` _itemstacks_4 _returnvalue_4 (- _output_4 1))
              (goto _label))
            (else
              ;[1 1 1] White Flower
              (if (== (`self.FlowerSelected`) (`|GetArrayItem` (`/Game/Interactables/BP_FlowerPlantation.FlowerMesh` (`self.CurrentSelectedPlanter`)) 3))
                (if (> _output 0)
                  (`KismetArrayLibrary.Array_Set` _itemstacks _returnvalue (- _output 1) true)
                  (goto _label))
                (else
                  (`KismetSystemLibrary.PrintString` "Collect Plant not adding to inventory" true true (struct :`R` 1.0 :`B` 0.138062 :`A` 1.0) 5.0))))))))))

(fn `PlanterRightBtn`
  (locals (PlantRight :type "StaticMeshComponent Object Reference"))
  (bind _currentselectedplanter (`self.CurrentSelectedPlanter`))
  (bind _plantright (`local.PlantRight`))
  (bind _flowermesh (`/Game/Interactables/BP_FlowerPlantation.FlowerMesh` _currentselectedplanter))
  (`/Engine/EditorBlueprintResources/StandardMacros.IncrementInt` (`self.PlantCounter`)
    (:`  `
      (set `local.PlantRight` (`/Game/Interactables/BP_FlowerPlantation.Plant` _currentselectedplanter))
      (if (> (`self.PlantCounter`) 3)
        (bind _output_get (set `self.PlantCounter` 0))
        (`StaticMeshComponent.SetStaticMesh` _plantright (`|GetArrayItem` _flowermesh _output_get))
        (`PrimitiveComponent.SetMaterial` _plantright 0 "/Game/HologramShader/MI_MasterMeshHologram.MI_MasterMeshHologram")
        (else
          (`StaticMeshComponent.SetStaticMesh` _plantright (`|GetArrayItem` _flowermesh (`self.PlantCounter`)))
          (`PrimitiveComponent.SetMaterial` _plantright 0 "/Game/HologramShader/MI_MasterMeshHologram.MI_MasterMeshHologram")))
      (`KismetMaterialLibrary.SetScalarParameterValue` "/Game/HologramShader/MPC_Hologram.MPC_Hologram" "Activation" 1.0)
      (return))))

(fn `ResetPlantation`
  (bind _currentselectedplanter (`self.CurrentSelectedPlanter`))
  (`SceneComponent.SetVisibility` (`/Game/Interactables/BP_FlowerPlantation.Cylinder` _currentselectedplanter) true false)
  (set `/Game/Interactables/BP_FlowerPlantation.IsHologram` true _currentselectedplanter)
  (set `/Game/Interactables/BP_FlowerPlantation.Planted` false _currentselectedplanter))

(fn `Tablet`
  (params (A :type "Float (double-precision)") (A2 :type "Float (double-precision)"))
  (bind _tabletui1 (`self.TabletUI1`))
  (bind _tabletui1_2 (`self.TabletUI1`))
  (bind (_relativelocation_x _relativelocation_y _relativelocation_z) (`KismetMathLibrary.BreakVector` (`SceneComponent.RelativeLocation` (`self.Point2`))))
  (bind (_relativelocation_x_2 _relativelocation_y_2 _relativelocation_z_2) (`KismetMathLibrary.BreakVector` (`SceneComponent.RelativeLocation` _tabletui1)))
  (bind (_relativelocation_x_3 _relativelocation_y_3 _relativelocation_z_3) (`KismetMathLibrary.BreakVector` (`SceneComponent.RelativeLocation` (`self.Point1`))))
  (bind (_relativelocation_x_4 _relativelocation_y_4 _relativelocation_z_4) (`KismetMathLibrary.BreakVector` (`SceneComponent.RelativeLocation` _tabletui1_2)))
  (if (`self.OpenTablet`)
    (`SceneComponent.K2_SetRelativeLocation` _tabletui1_2 (`KismetMathLibrary.MakeVector` _relativelocation_x_4 _relativelocation_y_4 (`KismetMathLibrary.Lerp` _relativelocation_z_4 _relativelocation_z_3 (* A 2.0))) false false)
    (else
      (`SceneComponent.K2_SetRelativeLocation` _tabletui1 (`KismetMathLibrary.MakeVector` _relativelocation_x_2 _relativelocation_y_2 (`KismetMathLibrary.Lerp` _relativelocation_z_2 _relativelocation_z (* A2 2.0))) false false))))

(fn `ToggleHud`
  (params (_changeState :type Boolean))
  (`MoonFloristHUD.ToggleAlpha` (`self.HUD`) _changeState))

(fn `UserConstructionScript`)