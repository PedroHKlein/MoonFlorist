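; BP_BouquetMark is a Blueprint that displays the game manager's current bouquet as flower meshes on seven slot components.
; BouquetChange calls ClearBouquet, reads three rows from MyGameManager, and adds a static mesh component for each supported flower ID.
; Row and position pick the snap-attach slot in a 2-3-2 layout.
; ClearBouquet, also run by BouquetClear, only removes entries from each slot's returned child array, destroying no components.
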(event `self.ReceiveBeginPlay`
  (bind _outactors (`GameplayStatics.GetAllActorsOfClass` "/Script/MoonFlorist.MyGameManager"))
  (set `self.GameManager` (`|GetArrayItem` _outactors))
  (set `self.SlotArray` (`|MakeArray` (`self.Slot1`) (`self.Slot2`) (`self.Slot3`) (`self.Slot4`) (`self.Slot5`) (`self.Slot6`) (`self.Slot7`))))

(event `BouquetChange`
  (bind _flowermesh (`self.FlowerMesh`))
  (bind _flowermesh_2 (`self.FlowerMesh`))
  (bind _flowermesh_3 (`self.FlowerMesh`))
  (bind _rowindex (`self.RowIndex`))
  (bind _flowerpos (`self.FlowerPos`))
  (`self.ClearBouquet`)
  (bind _returnvalue (`MyGameManager.GetBouquet` (`self.GameManager`)))
  (for _index (range 1 4)
    (set `self.RowIndex` _index)
    (bind _returnvalue_2 (`MyBouquet.GetRow` _returnvalue _index))
    (for (_array_element _array_index) _returnvalue_2
      (set `self.FlowerPos` _array_index)
      (bind _returnvalue_3 (`MyFlower.GetFlowerID` _array_element))
      (bind _output_get (set `self.FlowerID` _returnvalue_3))
      (if (== _output_get 1)
        (bind _returnvalue_4 (`AddComponent|NODE_AddStaticMeshComponent-2`))
        (set `self.FlowerMesh` _returnvalue_4)
        (if (== _rowindex 1) :!label _label
          (if (== (`self.FlowerPos`) 0)
            (`SceneComponent.K2_AttachToComponent` _flowermesh (`self.Slot1`) "None" "SnapToTarget" "SnapToTarget" "SnapToTarget" true)
            (else
              (`SceneComponent.K2_AttachToComponent` _flowermesh (`self.Slot2`) "None" "SnapToTarget" "SnapToTarget" "SnapToTarget" true)))
          (elif (== _rowindex 2)
            (if (== _flowerpos 0)
              (`SceneComponent.K2_AttachToComponent` _flowermesh_2 (`self.Slot3`) "None" "SnapToTarget" "SnapToTarget" "SnapToTarget" true)
              (elif (== _flowerpos 1)
                (`SceneComponent.K2_AttachToComponent` _flowermesh_2 (`self.Slot4`) "None" "SnapToTarget" "SnapToTarget" "SnapToTarget" true)
                (else
                  (`SceneComponent.K2_AttachToComponent` _flowermesh_2 (`self.Slot5`) "None" "SnapToTarget" "SnapToTarget" "SnapToTarget" true))))
            (elif (== _rowindex 3)
              (if (== (`self.FlowerPos`) 0)
                (`SceneComponent.K2_AttachToComponent` _flowermesh_3 (`self.Slot6`) "None" "SnapToTarget" "SnapToTarget" "SnapToTarget" true)
                (else
                  (`SceneComponent.K2_AttachToComponent` _flowermesh_3 (`self.Slot7`) "None" "SnapToTarget" "SnapToTarget" "SnapToTarget" true))))))
        (elif (== _output_get 2)
          (bind _returnvalue_5 (`AddComponent|NODE_AddStaticMeshComponent-3`))
          (set `self.FlowerMesh` _returnvalue_5)
          (goto _label)
          (elif (== _output_get 3)
            (bind _returnvalue_6 (`AddComponent|NODE_AddStaticMeshComponent-4`))
            (set `self.FlowerMesh` _returnvalue_6)
            (goto _label)
            (elif (== _output_get 7)
              (bind _returnvalue_7 (`AddComponent|NODE_AddStaticMeshComponent-5`))
              (set `self.FlowerMesh` _returnvalue_7)
              (goto _label))))))))

(event `BouquetClear`
  (`self.ClearBouquet`))

(fn `ClearBouquet`
  (for _array_element (`self.SlotArray`)
    (`KismetArrayLibrary.Array_RemoveItem` (`SceneComponent.GetChildrenComponents` _array_element false))))

(fn `UpdateBouquet`)

(fn `UserConstructionScript`)