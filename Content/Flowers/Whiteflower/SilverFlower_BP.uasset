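; Silver flower Blueprint that grows in stages, resuming when watered.
; BeginPlay calls Setup, zeroes the skeletal mesh scale and starts GrowingTimeline, which drives scale at a variable play rate.
; A Pausing event track halts the timeline and animation rate until Tick sees Watered while Growing, then resumes both.
; Timeline updates clear Watered, and completion clears Growing to end further growth.
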(event `GrowAfterWatering`
  ;[1 1 1] Continue Growing, Reset the Anim Rate
  (set `self.AnimationRate` 1.0)
  (bind (_direction _scale) (`Timeline|GrowingTimeline` :!label _label)
    (:`Update`
      (`SceneComponent.SetRelativeScale3D` (`self.FlowerSKMesh`) (`KismetMathLibrary.Conv_DoubleToVector` _scale))
      (`TimelineComponent.SetPlayRate` (`self.GrowingTimeline`) (`self.PlayRate`))
      (set `self.Watered` false))
    (:`Finished`
      (set `self.Growing` false))
    (:`Pausing`
      ;[1 1 1] Pause Growing Animation
      (set `self.AnimationRate` 0.0)
      (goto _label :!via `Stop`))))

(event `self.ReceiveBeginPlay`
  (`self.Setup`)
  (`SceneComponent.SetRelativeScale3D` (`self.FlowerSKMesh`) (0.0 0.0 0.0))
  (goto _label :!via `PlayFromStart`))

(event `self.ReceiveTick`
  (params (DeltaSeconds :type "Float (single-precision)"))
  (if (and (`self.Watered`) (`self.Growing`))
    (`self.GrowAfterWatering`)))

(fn `UserConstructionScript`)