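; Golden flower actor that grows from zero scale, pauses when it needs water, and becomes collectable after blooming.
; GrowingTimeline drives skeletal mesh scale, and its Pausing event halts growth and animation until Tick sees the flower watered.
; When ready to bloom, Timeline_0 times the collect window, then desaturates two dynamic materials.
; Watering during desaturation restores color and collectability.
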(event `GrowAfterWatering`
  ;[1 1 1] Continue Growing, Reset the Anim Rate
  (set `self.AnimationRate` 1.0)
  (set `self.NeedWater` false)
  (bind (_direction _scale) (`Timeline|GrowingTimeline` :!label _label)
    (:`Update`
      (`SceneComponent.SetRelativeScale3D` (`self.FlowerSKMesh`) (`KismetMathLibrary.Conv_DoubleToVector` _scale))
      (`TimelineComponent.SetPlayRate` (`self.GrowingTimeline`) (`self.PlayRate`)))
    (:`Finished`
      (set `self.Growing` false)
      (set `self.Watered` false))
    (:`Pausing`
      ;[1 1 1] Pause Growing Animation
      (set `self.AnimationRate` 0.0)
      (set `self.Watered` false)
      (set `self.NeedWater` true)
      (goto _label :!via `Stop`))))

(event `self.ReceiveBeginPlay`
  (`self.Setup`)
  (`SceneComponent.SetRelativeScale3D` (`self.FlowerSKMesh`) (0.0 0.0 0.0))
  (goto _label :!via `PlayFromStart`))

(event `self.ReceiveTick`
  (params (DeltaSeconds :type "Float (single-precision)"))
  (if (and (`self.Watered`) (`self.Growing`))
    (`self.GrowAfterWatering`)
    (if (`self.ReadyToBloom`)
      (`self.AfterBloom`))))

(event `AfterBloom`
  (bind (_direction _desaturationrate) (`Timeline|Timeline_0`)
    (:`Update`
      (if (`self.StartDesaturation`)
        (`MaterialInstanceDynamic.SetScalarParameterValue` (`self.DM_FirstElement`) "Desaturation" _desaturationrate)
        (`MaterialInstanceDynamic.SetScalarParameterValue` (`self.DM_SecondElement`) "Desaturation" _desaturationrate)
        (if (`self.Watered`)
          (set `self.ReadyToCollect` true)
          (`MaterialInstanceDynamic.SetScalarParameterValue` (`self.DM_FirstElement`) "Desaturation" 0.0)
          (`MaterialInstanceDynamic.SetScalarParameterValue` (`self.DM_SecondElement`) "Desaturation" 0.0)
          (set `self.NeedWater` false))))
    (:`1 Minute`
      (set `self.ReadyToCollect` true))
    (:`Begin Desaturation`
      (set `self.ReadyToCollect` false)
      (`KismetSystemLibrary.PrintString` "it begins")
      (set `self.StartDesaturation` true)
      (set `self.NeedWater` true))))

(fn `UserConstructionScript`)