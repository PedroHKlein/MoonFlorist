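; BP_FlowerBloom is a flower actor that grows from nothing when play begins.
; BeginPlay clears the bloom and collect flags, zeroes the mesh scale, and plays the grow animation once while GrowingTimeline drives the scale.
; When the timeline finishes, it sets ReadyToBloom and prints a debug message.
; PlantFlower is an empty event, and nothing here sets ReadyToCollect to true.
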(event `self.ReceiveBeginPlay`
  (set `self.ReadyToBloom` false)
  (set `self.ReadyToCollect` false)
  (`SceneComponent.SetRelativeScale3D` (`self.Flower_grow_anim`) (0.0 0.0 0.0))
  (`SkeletalMeshComponent.PlayAnimation` (`self.Flower_grow_anim`) "/Game/Flowers/Flower_grow_anim.Flower_Grow_anim" false)
  (bind (_direction _scale) (`Timeline|Growing Timeline` :!via `PlayFromStart`)
    (:`Update`
      (`SceneComponent.SetRelativeScale3D` (`self.Flower_grow_anim`) (`KismetMathLibrary.Conv_DoubleToVector` _scale)))
    (:`Finished`
      (set `self.ReadyToBloom` true)
      (`KismetSystemLibrary.PrintString` "Finished Growiing"))))

(event `Plant Flower`)

(fn `UserConstructionScript`)