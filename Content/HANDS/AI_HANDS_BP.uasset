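; AI Blueprint for the hands, which switches them to the Park state when the game manager signals that they can deliver.
; BeginPlay caches the first MyGameManager actor found in the level.
; Tick polls its HandsCanDeliver flag and calls SetHandsState with Park on every frame it is true.
; Nothing here resets the state, as the Patrolling call is left unconnected.
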(event `self.ReceiveBeginPlay`
  (`parent.ReceiveBeginPlay`)
  (bind _outactors (`GameplayStatics.GetAllActorsOfClass` "/Script/MoonFlorist.MyGameManager"))
  (set `self.GameManager` (`|GetArrayItem` _outactors)))

(event `self.ReceiveTick`
  (params (DeltaSeconds :type "Float (single-precision)"))
  (bind _gamemanager (`self.GameManager`))
  (`parent.ReceiveTick` DeltaSeconds)
  (`/Engine/EditorBlueprintResources/StandardMacros.IsValid` _gamemanager
    (:`Is Valid`
      (if (`MyGameManager.HandsCanDeliver` _gamemanager)
        (`self.SetHandsState` "HS_Park")))))

(fn `UserConstructionScript`)