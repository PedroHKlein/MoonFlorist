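; BP_FlowerBloom is a flower Blueprint that grows into view when play begins.
; BeginPlay sets StaticMesh to zero relative scale, then plays GrowingTimeline, whose Scale track drives the relative scale of both the Flower component and StaticMesh.
; PlantFlower is an empty event, and the Flower_grow_anim playback nodes are disconnected, so the bloom relies on scaling alone.
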(event `self.ReceiveBeginPlay`
  (`SceneComponent.SetRelativeScale3D` (`self.StaticMesh`) (0.0 0.0 0.0))
  (bind (_direction _scale) (`Timeline|Growing Timeline`)
    (:`Update`
      (`SceneComponent.SetRelativeScale3D` (`self.Flower`) (`KismetMathLibrary.Conv_DoubleToVector` _scale))
      (`SceneComponent.SetRelativeScale3D` (`self.StaticMesh`) (`KismetMathLibrary.Conv_DoubleToVector` _scale)))))

(event `Plant Flower`)

(fn `UserConstructionScript`)