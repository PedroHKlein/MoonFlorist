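; Spline-driven mesh Blueprint in the vegetation folder that repeats one static mesh along a spline.
; The Construction Script adds a spline mesh component per Spacing interval, with start and end offsets adjusting each segment's endpoints.
; Tangents follow spline direction, scaled down on the last segment by the leftover length.
; Each segment takes spline scale at both ends, its midpoint up vector, and end rolls relative to that midpoint to follow twist.
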(fn `UserConstructionScript`
  (bind (_remainder _returnvalue) (`KismetMathLibrary.FMod` (`SplineComponent.GetSplineLength` (`self.Spline1`)) (`self.Spacing`)))
  (bind _returnvalue_2 (`KismetMathLibrary.NegateRotator` (`SplineComponent.GetRotationAtDistanceAlongSpline` (`self.Spline1`) (`self.MiddleDistance`) "Local")))
  (for _index (range (+ _returnvalue 1))
    (bind _output_get (set `self.Index` _index))
    (set `self.FinalTangentScale` (select `bool` (== _output_get _returnvalue) :`false` (`self.TangentScale`) :`true` (* (/ _remainder (`self.Spacing`)) (`self.TangentScale`))))
    (bind _output_get_2 (set `self.StartDistance` (* (`self.Index`) (`self.Spacing`))))
    (set `self.MiddleDistance` (+ _output_get_2 (* (`self.Spacing`) 0.5)))
    (set `self.EndDistance` (+ (`self.StartDistance`) (`self.Spacing`)))
    (bind _returnvalue_3 (`AddComponent|NODE_AddSplineMeshComponent-0`))
    (bind _output_get_3 (set `self.Spline_Mesh` _returnvalue_3))
    (`SplineMeshComponent.SetStartAndEnd` _output_get_3 (`SplineComponent.GetLocationAtDistanceAlongSpline` (`self.Spline1`) (- (`self.StartDistance`) (`self.StartOffset`)) "Local") (* (`SplineComponent.GetDirectionAtDistanceAlongSpline` (`self.Spline1`) (`self.StartDistance`) "Local") (`self.FinalTangentScale`)) (`SplineComponent.GetLocationAtDistanceAlongSpline` (`self.Spline1`) (+ (`self.EndDistance`) (`self.EndOffset`)) "Local") (* (`SplineComponent.GetDirectionAtDistanceAlongSpline` (`self.Spline1`) (`self.EndDistance`) "Local") (`self.FinalTangentScale`)) true)
    (`SplineMeshComponent.SetStartScale` (`self.Spline_Mesh`) (`KismetMathLibrary.MakeVector2D` (.y (`SplineComponent.GetScaleAtDistanceAlongSpline` (`self.Spline1`) (`self.StartDistance`))) (.z (`SplineComponent.GetScaleAtDistanceAlongSpline` (`self.Spline1`) (`self.StartDistance`)))) true)
    (`SplineMeshComponent.SetEndScale` (`self.Spline_Mesh`) (`KismetMathLibrary.MakeVector2D` (.y (`SplineComponent.GetScaleAtDistanceAlongSpline` (`self.Spline1`) (`self.EndDistance`))) (.z (`SplineComponent.GetScaleAtDistanceAlongSpline` (`self.Spline1`) (`self.EndDistance`)))) true)
    (`SplineMeshComponent.SetSplineUpDir` (`self.Spline_Mesh`) (`SplineComponent.GetUpVectorAtDistanceAlongSpline` (`self.Spline1`) (`self.MiddleDistance`) "World") true)
    (`SplineMeshComponent.SetStartRoll` (`self.Spline_Mesh`) (`KismetMathLibrary.DegreesToRadians` (.roll (`KismetMathLibrary.ComposeRotators` (`SplineComponent.GetRotationAtDistanceAlongSpline` (`self.Spline1`) (`self.StartDistance`) "Local") _returnvalue_2))) true)
    (`SplineMeshComponent.SetEndRoll` (`self.Spline_Mesh`) (`KismetMathLibrary.DegreesToRadians` (.roll (`KismetMathLibrary.ComposeRotators` (`SplineComponent.GetRotationAtDistanceAlongSpline` (`self.Spline1`) (`self.EndDistance`) "Local") _returnvalue_2))) true)
    (`StaticMeshComponent.SetStaticMesh` (`self.Spline_Mesh`) (`self.Mesh`))))