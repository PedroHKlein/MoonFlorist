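; Base actor for interactables that shows a floating name label when the player is nearby.
; Every Tick it compares its distance to player character 0 against a fixed range, toggles the FloatingText widget component, and yaws it toward the player while visible.
; GetInteractableName copies the actor's Name into the FloatingText widget, though nothing in this Blueprint calls it.
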(event `self.ReceiveBeginPlay`)

(event `self.ReceiveTick`
  (params (DeltaSeconds :type "Float (single-precision)"))
  (`self.ToggleVisiblity-FloatingText(Actor)` 200.0))

(fn `GetInteractableName`
  (bind _asfloating_text (cast `/Game/User_Interface/FloatingText` (`WidgetComponent.GetUserWidgetObject` (`self.FloatingText`)))
    (:`then`
      (set `/Game/User_Interface/FloatingText.Interactable Name` (`KismetTextLibrary.Conv_StringToText` (`self.Name`)) _asfloating_text))
    (:`CastFailed`
      (`KismetSystemLibrary.PrintString` "Cast to Floating Text Failed" true true (struct :`R` 1.0 :`B` 0.247108 :`A` 1.0) 5.0))))

(fn `ToggleVisiblity-FloatingText(Actor)`
  (params (Distance :type "Float (double-precision)"))
  (bind (_returnvalue_roll _returnvalue_pitch _returnvalue_yaw) (`KismetMathLibrary.BreakRotator` (`KismetMathLibrary.FindLookAtRotation` (`self.K2_GetActorLocation`) (`self.K2_GetActorLocation` (`GameplayStatics.GetPlayerCharacter` 0)))))
  (bind _returnvalue (<= (`KismetMathLibrary.VSize` (- (`self.K2_GetActorLocation`) (`self.K2_GetActorLocation` (`GameplayStatics.GetPlayerCharacter` 0)))) Distance))
  (if _returnvalue
    (`SceneComponent.SetVisibility` (`self.FloatingText`) _returnvalue false)
    (`SceneComponent.K2_SetWorldRotation` (`self.FloatingText`) (`KismetMathLibrary.MakeRotator` 0.0 0.0 _returnvalue_yaw) false false)
    (else
      (`SceneComponent.SetVisibility` (`self.FloatingText`) _returnvalue false))))

(fn `UserConstructionScript`)