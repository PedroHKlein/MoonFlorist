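; BedroomPanel_BP is a bedroom panel whose hours and minutes emissive colors reflect whether the sliding window is open.
; On BeginPlay it caches the first SlidingWindow_BP found in the level, after running the parent logic.
; Each Tick, if that reference is valid, it reads the window's Open flag and passes one of two color pairs to DynamicMaterialChanging for both dynamic materials.
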(event `self.ReceiveBeginPlay`
  (`parent.ReceiveBeginPlay`)
  (bind _outactors (`GameplayStatics.GetAllActorsOfClass` "/Game/Interactables/SlidingWindow_BP.SlidingWindow_BP_C"))
  (set `self.sliding window` (`|GetArrayItem` _outactors)))

(event `self.ReceiveTick`
  (params (DeltaSeconds :type "Float (single-precision)"))
  (bind _sliding_window (`self.sliding window`))
  (bind _dynamicmaterialhours (`self.DynamicMaterialHours`))
  (bind _dynamicmaterialminutes (`self.DynamicMaterialMinutes`))
  (`parent.ReceiveTick` 0.0)
  (`/Engine/EditorBlueprintResources/StandardMacros.IsValid` _sliding_window
    (:`Is Valid`
      (if (`SlidingWindow.Open` _sliding_window)
        (`self.DynamicMaterialChanging` _dynamicmaterialhours null (`self.Colour2_0`) (`self.Colour2_1`))
        (`self.DynamicMaterialChanging` _dynamicmaterialminutes null (`self.Colour2_0`) (`self.Colour2_1`))
        (else
          (`self.DynamicMaterialChanging` _dynamicmaterialhours null (`self.Colour1_0`) (`self.Colour1_1`))
          (`self.DynamicMaterialChanging` _dynamicmaterialminutes null (`self.Colour1_0`) (`self.Colour1_1`)))))))

(fn `UserConstructionScript`)