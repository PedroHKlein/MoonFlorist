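; Day/night material switcher Blueprint that changes a dynamic material's look based on whether a sliding window is open.
; On BeginPlay it caches the first SlidingWindow_BP found in the level.
; Every Tick it calls the parent Tick, then polls the window's Open flag and passes DynamicMaterialSwitching the off texture and emission color pair when open, or the on set when closed.
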(event `self.ReceiveBeginPlay`
  (bind _outactors (`GameplayStatics.GetAllActorsOfClass` "/Game/Interactables/SlidingWindow_BP.SlidingWindow_BP_C"))
  (set `self.SlidingWindow` (`|GetArrayItem` _outactors)))

(event `self.ReceiveTick`
  (params (DeltaSeconds :type "Float (single-precision)"))
  (bind _dm (`self.DM`))
  (`parent.ReceiveTick` DeltaSeconds)
  (if (`SlidingWindow.Open` (`self.SlidingWindow`))
    (`self.DynamicMaterialSwitching` _dm "/Game/Materials/Textures/T_Off.T_Off" (`self.Colour2_0`) (`self.Colour2_1`))
    (else
      (`self.DynamicMaterialSwitching` _dm "/Game/Materials/Textures/T_On.T_On" (`self.Colour1_0`) (`self.Colour1_1`)))))

(fn `UserConstructionScript`)