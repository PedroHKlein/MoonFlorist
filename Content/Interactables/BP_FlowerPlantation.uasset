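; Interactable flower plantation where the player picks one of four flowers from a rotating hologram preview, plants it and later collects it.
; Scroll inputs or buttons cycle meshes, with a timeline driving the hologram's Material Parameter Collection.
; Planting removes the matching seed from PlayerStorage, restores real materials, scales the plant via timeline and enables collection after a delay.
; Collecting adds the flower to storage, matched by enum name, then resets to hologram mode.
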(event `self.ReceiveBeginPlay`
  (`KismetMaterialLibrary.CreateDynamicMaterialInstance` "/Game/HologramShader/MI_MasterHologram.MI_MasterHologram")
  (`KismetMaterialLibrary.CreateDynamicMaterialInstance` "/Game/HologramShader/MI_MasterMeshHologram.MI_MasterMeshHologram")
  (`self.EnableInput` (`GameplayStatics.GetPlayerController` 0))
  (`self.GetInteractableName`)
  (`SceneComponent.SetVisibility` (`self.ConfirmBtn`) false false)
  (`SceneComponent.SetVisibility` (`self.Widget`) false false)
  (bind _asbp_moon_florist_character (cast `/Game/BP_MoonFloristCharacter` (`GameplayStatics.GetPlayerCharacter` 0)))
  (set `self.Player` _asbp_moon_florist_character))

(event `self.ReceiveTick`
  (params (DeltaSeconds :type "Float (single-precision)"))
  (`parent.ReceiveTick` DeltaSeconds)
  (if (`self.IsHologram`)
    (`SceneComponent.K2_AddLocalRotation` (`self.Plant`) (* (`self.Rotation Axis`) (`self.Rotation Speed`)) false false))
  (`PrimitiveComponent.SetRenderCustomDepth` (`self.Incubator_rough`) (`self.ShowOutline`)))

(event `Plant_BTN`
  (set `self.IsHologram` false)
  (set `self.Planted` true)
  (`self.Planting`)
  (bind (_direction _scale) (`Timeline|Timeline_1` :!via `PlayFromStart`)
    (:`Update`
      (`SceneComponent.SetRelativeScale3D` (`self.Plant`) (`KismetMathLibrary.Conv_DoubleToVector` _scale))
      (`self.FinishGrowth`)
      (`KismetSystemLibrary.Delay` (`self.TotalPlantationTime`))
      (`KismetSystemLibrary.PrintString` "Plant Finished")
      (set `/Game/BP_MoonFloristCharacter.CanCollect` true (`self.Player`)))))

(event `InputAction|ScrollLeft`
  (params (Key :type "Key Structure"))
  ;[1 1 1] Keyboard
  (:`Pressed`
    (if (and (`MoonFloristCharacter.Interacting` (`self.Player`)) (`self.IsHologram`)) :!label _label
      (`SceneComponent.SetVisibility` (`self.Cylinder`) true false)
      (`self.LeftBtn`)
      (bind (_direction _activate) (`Timeline|Timeline_2` :!via `PlayFromStart` :!label _label_2)
        (:`Update`
          (`KismetMaterialLibrary.SetScalarParameterValue` "/Game/HologramShader/MPC_Hologram.MPC_Hologram" "Activation" _activate))))))

(event `Lft_BTN`
  ;[1 1 1] Keyboard
  (goto _label))

(event `InputAction|ScrollRight`
  (params (Key :type "Key Structure"))
  ;[1 1 1] Keyboard
  (:`Pressed`
    (if (and (`MoonFloristCharacter.Interacting` (`self.Player`)) (`self.IsHologram`)) :!label _label_3
      (`SceneComponent.SetVisibility` (`self.Cylinder`) true false)
      (`self.RightBtn`)
      (goto _label_2 :!via `PlayFromStart`))))

(event `Rgt_BTN`
  ;[1 1 1] Keyboard
  (goto _label_3))

(event `Collect_BTN`
  (`self.PlantCollect`)
  (`KismetSystemLibrary.Delay` 2.0)
  (`self.Reset`))

(fn `CollectingFlower`
  (params (Enumerator :type "EItems Enum" :default "Scarletflower"))
  (bind _playerstorage (`MoonFloristCharacter.PlayerStorage` (`self.Player`)))
  (for _array_element (`Storage.StorageArray` _playerstorage)
    (bind _returnvalue (`Item.GetName` _array_element))
    (if (== _returnvalue (`KismetStringLibrary.Conv_StringToName` (`|GetEnumeratorNameAsString` Enumerator)))
      (`Storage.IncreaseStacks` _playerstorage 1 _array_element)
      (return))))

(fn `FinishGrowth`
  (`StaticMeshComponent.SetStaticMesh` (`self.Plant`) (`self.Flower Selected`))
  (return))

(fn `LeftBtn`
  (bind _plant (`self.Plant`))
  (bind _flowermesh (`self.FlowerMesh`))
  (`/Engine/EditorBlueprintResources/StandardMacros.DecrementInt` (`self.PlantCounter`)
    (:`  `
      (if (< (`self.PlantCounter`) 0)
        (bind _output_get (set `self.PlantCounter` 3))
        (`StaticMeshComponent.SetStaticMesh` _plant (`|GetArrayItem` _flowermesh _output_get))
        (`PrimitiveComponent.SetMaterial` _plant 0 "/Game/HologramShader/MI_MasterMeshHologram.MI_MasterMeshHologram")
        (else
          (`StaticMeshComponent.SetStaticMesh` _plant (`|GetArrayItem` _flowermesh (`self.PlantCounter`)))
          (`PrimitiveComponent.SetMaterial` _plant 0 "/Game/HologramShader/MI_MasterMeshHologram.MI_MasterMeshHologram")))
      (`KismetMaterialLibrary.SetScalarParameterValue` "/Game/HologramShader/MPC_Hologram.MPC_Hologram" "Activation" 1.0)
      (return))))

(fn `PlantCollect`
  ;[1 0 0] Red Flower
  (if (== (`self.Flower Selected`) (`|GetArrayItem` (`self.FlowerMesh`)))
    (`self.CollectingFlower` "Scarletflower")
    (`StaticMeshComponent.SetStaticMesh` (`self.Plant`) null :!label _label)
    (set `/Game/BP_MoonFloristCharacter.CanCollect` false (`self.Player`))
    (return)
    (else
      ;[0 0.1291 1] Blue Flower
      (if (== (`self.Flower Selected`) (`|GetArrayItem` (`self.FlowerMesh`) 1))
        (`self.CollectingFlower` "Cobaltflower")
        (goto _label)
        (else
          ;[1 0.8718 0] Yellow Flower
          (if (== (`self.Flower Selected`) (`|GetArrayItem` (`self.FlowerMesh`) 2))
            (`self.CollectingFlower` "Goldenflower")
            (goto _label)
            (else
              ;[1 1 1] White Flower
              (if (== (`self.Flower Selected`) (`|GetArrayItem` (`self.FlowerMesh`) 3))
                (`self.CollectingFlower` "Silverflower")
                (goto _label)))))))))

(fn `Planting`
  (bind _plant (`self.Plant`))
  (set `self.Flower Selected` (`StaticMeshComponent.StaticMesh` (`self.Plant`)))
  ;[1 0 0] Red Flower
  (if (== (`self.Flower Selected`) (`|GetArrayItem` (`self.FlowerMesh`)))
    (`self.PlantingFlower` "Scarletseed")
    (`PrimitiveComponent.SetMaterial` _plant 0 (`StaticMesh.GetMaterial` (`self.Flower Selected`) 0) :!label _label)
    (if (> (`PrimitiveComponent.GetNumMaterials` _plant) 1)
      (`PrimitiveComponent.SetMaterial` (`self.Plant`) 1 (`StaticMesh.GetMaterial` (`self.Flower Selected`) 1)))
    (`SceneComponent.SetVisibility` (`self.Cylinder`) false false)
    (return)
    (else
      ;[0 0.1291 1] Blue Flower
      (if (== (`self.Flower Selected`) (`|GetArrayItem` (`self.FlowerMesh`) 1))
        (`self.PlantingFlower` "Cobaltseed")
        (goto _label)
        (else
          ;[1 0.8718 0] Yellow Flower
          (if (== (`self.Flower Selected`) (`|GetArrayItem` (`self.FlowerMesh`) 2))
            (`self.PlantingFlower` "Goldenseed")
            (goto _label)
            (else
              ;[1 1 1] White Flower
              (if (== (`self.Flower Selected`) (`|GetArrayItem` (`self.FlowerMesh`) 3))
                (`self.PlantingFlower` "Silverseed")
                (goto _label)))))))))

(fn `PlantingFlower`
  (params (Enumerator :type "EItems Enum" :default "Scarletflower"))
  (bind _playerstorage (`MoonFloristCharacter.PlayerStorage` (`self.Player`)))
  (for _array_element (`Storage.StorageArray` _playerstorage)
    (bind _returnvalue (`Item.GetName` _array_element))
    (if (== _returnvalue (`KismetStringLibrary.Conv_StringToName` (`|GetEnumeratorNameAsString` Enumerator)))
      (`Storage.DecreaseStacks` _playerstorage 1 _array_element))))

(fn `Reset`
  (bind _plant (`self.Plant`))
  (`SceneComponent.SetVisibility` (`self.Cylinder`) true false)
  (`SceneComponent.SetVisibility` _plant true false)
  (set `self.IsHologram` true)
  (set `self.Planted` false)
  (`StaticMeshComponent.SetStaticMesh` _plant "/Game/Flowers/SM_Flower_Red.SM_Flower_Red")
  (`PrimitiveComponent.SetMaterial` _plant 0 "/Game/HologramShader/MI_MasterMeshHologram.MI_MasterMeshHologram")
  (if (> (`PrimitiveComponent.GetNumMaterials` _plant) 1)
    (`PrimitiveComponent.SetMaterial` _plant 1 "/Game/HologramShader/MI_MasterMeshHologram.MI_MasterMeshHologram"))
  (`KismetMaterialLibrary.SetScalarParameterValue` "/Game/HologramShader/MPC_Hologram.MPC_Hologram" "Activation")
  (return))

(fn `RightBtn`
  (bind _flowermesh (`self.FlowerMesh`))
  (bind _plant (`self.Plant`))
  (`/Engine/EditorBlueprintResources/StandardMacros.IncrementInt` (`self.PlantCounter`)
    (:`  `
      (if (> (`self.PlantCounter`) 3)
        (bind _output_get (set `self.PlantCounter` 0))
        (`StaticMeshComponent.SetStaticMesh` _plant (`|GetArrayItem` _flowermesh _output_get))
        (`PrimitiveComponent.SetMaterial` _plant 0 "/Game/HologramShader/MI_MasterMeshHologram.MI_MasterMeshHologram")
        (else
          (`StaticMeshComponent.SetStaticMesh` _plant (`|GetArrayItem` _flowermesh (`self.PlantCounter`)))
          (`PrimitiveComponent.SetMaterial` _plant 0 "/Game/HologramShader/MI_MasterMeshHologram.MI_MasterMeshHologram")))
      (`KismetMaterialLibrary.SetScalarParameterValue` "/Game/HologramShader/MPC_Hologram.MPC_Hologram" "Activation" 1.0)
      (return))))

(fn `UserConstructionScript`
  (`self.Reset`))