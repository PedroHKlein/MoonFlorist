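; Delivery terminal interactable that displays the bouquet capsule and completes the player's flower order.
; Tick polls the game manager's ConstructCapsule flag to spawn a capsule, load it with the current bouquet and snap it to the stand.
; A MakeCapsule flag triggers order completion, tablet text reset, a CosmoCoin award and capsule destruction.
; ShowOutline toggles custom depth rendering on the stand meshes, also every tick.
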(event `self.ReceiveBeginPlay`
  (`parent.ReceiveBeginPlay`)
  (bind _outactors (`GameplayStatics.GetAllActorsOfClass` "/Script/MoonFlorist.MyGameManager"))
  (set `self.GameManager` (`|GetArrayItem` _outactors))
  (bind _asbp_moon_florist_character (cast `/Game/BP_MoonFloristCharacter` (`GameplayStatics.GetPlayerCharacter` 0)))
  (set `self.PlayerRef` _asbp_moon_florist_character)
  (bind _foundwidgets (`WidgetBlueprintLibrary.GetAllWidgetsOfClass` "/Game/User_Interface/Tablet/TabletUI.TabletUI_C" false))
  (set `self.TabUI` (`|GetArrayItem` _foundwidgets)))

(event `self.ReceiveTick`
  (params (DeltaSeconds :type "Float (single-precision)"))
  (bind _playerref (`self.PlayerRef`))
  (bind _tabui (`self.TabUI`))
  (bind _gamemanager (`self.GameManager`))
  (`parent.ReceiveTick` DeltaSeconds)
  (`/Engine/EditorBlueprintResources/StandardMacros.IsValid` _gamemanager
    (:`Is Valid`
      (if (`MyGameManager.ConstructCapsule` _gamemanager)
        (bind _returnvalue (`|SpawnActorFromClass` "/Game/Interactables/BouquetCapsule_BP.BouquetCapsule_BP_C" (`SceneComponent.K2_GetComponentToWorld` (`self.Position1`)) "Undefined" "OverrideRootScale" self null))
        (bind _returnvalue_2 (`MyGameManager.GetBouquet` _gamemanager))
        (`BouquetCapsule.StoreBouquetInCap` _returnvalue _returnvalue_2)
        (set `MyGameManager.ConstructCapsule` false _gamemanager)
        (`self.K2_AttachToComponent` _returnvalue (`self.Position1`) "MagnetSocket" "SnapToTarget" "SnapToTarget" "KeepWorld" true)))
    (:`Is Not Valid`
      _))
  (if (`self.ShowOutline`)
    (`PrimitiveComponent.SetRenderCustomDepth` (`self.StandBase`) true)
    (`PrimitiveComponent.SetRenderCustomDepth` (`self.StandMagnet`) true)
    (`PrimitiveComponent.SetRenderCustomDepth` (`self.StandBaseArm`) true)
    (`PrimitiveComponent.SetRenderCustomDepth` (`self.Cylinder2`) true)
    (`PrimitiveComponent.SetRenderCustomDepth` (`self.Cylinder`) true)
    (`PrimitiveComponent.SetRenderCustomDepth` (`self.StandBody`) true)
    (else
      (`PrimitiveComponent.SetRenderCustomDepth` (`self.Cylinder`) false)
      (`PrimitiveComponent.SetRenderCustomDepth` (`self.Cylinder2`) false)
      (`PrimitiveComponent.SetRenderCustomDepth` (`self.StandBaseArm`) false)
      (`PrimitiveComponent.SetRenderCustomDepth` (`self.StandMagnet`) false)
      (`PrimitiveComponent.SetRenderCustomDepth` (`self.StandBase`) false)
      (`PrimitiveComponent.SetRenderCustomDepth` (`self.StandBody`) false)))
  (if (`self.MakeCapsule`)
    (`MyGameManager.CompleteOrder` (`self.GameManager`))
    (bind _returnvalue_3 (`MyGameManager.GetMoney` (`self.GameManager`)))
    (`KismetSystemLibrary.PrintString` (`KismetStringLibrary.Conv_IntToString` _returnvalue_3))
    (`KismetSystemLibrary.PrintString` "Moolah After")
    (bind _foundwidgets (`WidgetBlueprintLibrary.GetAllWidgetsOfClass` "/Game/User_Interface/Tablet/TabletUI.TabletUI_C" false))
    (set `self.TabUI` (`|GetArrayItem` _foundwidgets))
    (`/Game/User_Interface/Tablet/TabletUI.Reset Order Text` _tabui)
    (`/Game/User_Interface/Tablet/TabletUI.Reset Feedback Text` _tabui)
    (set `self.MakeCapsule` false)
    (set `MoonFloristCharacter.CosmoCoins` (+ (`MoonFloristCharacter.CosmoCoins` _playerref) 1) _playerref)
    (`/Engine/EditorBlueprintResources/StandardMacros.IsValid` _returnvalue
      (:`Is Valid`
        (`self.K2_DestroyActor` _returnvalue)))))

(fn `UserConstructionScript`)