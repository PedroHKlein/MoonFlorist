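; Interactable planting area for the Moon Florist player, with its own orbit camera and an interaction widget.
; Tick drives the custom-depth outline from ShowOutline and shows the widget only while the player is interacting with this actor.
; MoveRight input yaws the spring arm at RotateRate and re-aims the camera at the planting area.
; BeginPlay caches the player character and the arm's initial yaw, which is not read in these graphs.
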(event `self.ReceiveBeginPlay`
  (bind (_returnvalue_roll _returnvalue_pitch _returnvalue_yaw) (`KismetMathLibrary.BreakRotator` (`SceneComponent.K2_GetComponentRotation` (`self.SpringArm`))))
  (set `self.InitalZ` _returnvalue_yaw)
  (bind _asbp_moon_florist_character (cast `/Game/BP_MoonFloristCharacter` (`GameplayStatics.GetPlayerCharacter` 0)))
  (set `self.PlayerRef_0` _asbp_moon_florist_character))

(event `self.ReceiveTick`
  (params (DeltaSeconds :type "Float (single-precision)"))
  (bind _playerref_0 (`self.PlayerRef_0`))
  (bind _widgetcomp (`self.WidgetComp`))
  (`parent.ReceiveTick` DeltaSeconds)
  (`PrimitiveComponent.SetRenderCustomDepth` (`self.PlantingArea`) (`self.ShowOutline`))
  (if (and (`MoonFloristCharacter.Interacting` _playerref_0) (== (`MoonFloristCharacter.CurrentInteractActor` _playerref_0) self))
    (`SceneComponent.SetVisibility` _widgetcomp true false)
    (else
      (`SceneComponent.SetVisibility` _widgetcomp false false))))

(event `InputAxis|MoveRight`
  (params (AxisValue :type "Float (single-precision)"))
  (`SceneComponent.K2_SetWorldRotation` (`self.SpringArm`) (`KismetMathLibrary.MakeRotator` (.roll (`SceneComponent.K2_GetComponentRotation` (`self.SpringArm`))) (.pitch (`SceneComponent.K2_GetComponentRotation` (`self.SpringArm`))) (+ (* AxisValue (`GameplayStatics.GetWorldDeltaSeconds`) (`self.RotateRate`) -1.0) (.yaw (`SceneComponent.K2_GetComponentRotation` (`self.SpringArm`))))) true false)
  (`SceneComponent.K2_SetWorldRotation` (`self.Camera`) (`KismetMathLibrary.FindLookAtRotation` (`SceneComponent.K2_GetComponentLocation` (`self.Camera`)) (`SceneComponent.K2_GetComponentLocation` (`self.PlantingArea`))) false false))

(fn `UserConstructionScript`)