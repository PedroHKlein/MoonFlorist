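; BP_RandomMesh is an actor that shows one static mesh picked from its Meshes array, adding visual variety to placed instances.
; The construction script uses MeshID when SetMeshID is on, otherwise it rolls a random index limited to the first three entries, stores it as HiddenMeshID and applies that mesh.
; The random choice is unseeded, so it can change whenever construction reruns; the event graph has no active logic.
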(fn `UserConstructionScript`
  (if (`self.Set Mesh ID?`)
    (set `self.Hidden Mesh ID` (`self.Mesh ID`))
    (else
      (set `self.Hidden Mesh ID` (`KismetMathLibrary.RandomIntegerInRange` 0 2))))
  (`StaticMeshComponent.SetStaticMesh` (`self.StaticMesh`) (`|GetArrayItem` (`self.Meshes`) (`self.Hidden Mesh ID`))))