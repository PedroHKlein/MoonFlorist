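; BP_MoonFloristHUD is the Moon Florist HUD Blueprint that creates the game's main UI widgets on BeginPlay and keeps references to them.
; The storage window is added to the viewport hidden, the checklist is added normally, and notifications are added at a negative Z-order.
; The order list widget is created and stored but not added to the viewport here.
; A disconnected tutorial box test never runs.
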(event `self.ReceiveBeginPlay`
  (bind _returnvalue (`GameplayStatics.GetPlayerController` 0))
  (bind _returnvalue_2 (`|CreateWidget` "/Game/User_Interface/Storage/StorageWindow.StorageWindow_C"))
  (bind _output_get (set `self.StorageUI` _returnvalue_2))
  (`Widget.SetVisibility` _output_get "Hidden")
  (`UserWidget.AddToViewport` _output_get 0)
  (bind _returnvalue_3 (`|CreateWidget` "/Game/User_Interface/OrderList/OrderList_Widget.OrderList_Widget_C" _returnvalue))
  (set `self.OrderListUI` _returnvalue_3)
  (bind _returnvalue_4 (`|CreateWidget` "/Game/User_Interface/Checklist/Checklist.Checklist_C" _returnvalue))
  (bind _output_get_2 (set `self.NewVar_0` _returnvalue_4))
  (`UserWidget.AddToViewport` _output_get_2 0)
  (bind _returnvalue_5 (`|CreateWidget` "/Game/User_Interface/Notifications/Notification_widget.Notification_widget_C" _returnvalue))
  (bind _output_get_3 (set `self.Notification UI` _returnvalue_5))
  (`UserWidget.AddToViewport` _output_get_3 -10))

(fn `UserConstructionScript`)