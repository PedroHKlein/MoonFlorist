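; Notification_Collision_BP is a one-shot trigger volume that shows a notification when the player walks into it.
; When its box collision begins overlapping, it checks that the other actor is the first BP_MoonFloristCharacter in the level.
; It then finds MyGameManager, passes it the configured Notification and Time through AddNotification, and destroys itself.
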(event `self.BoxCollision.OnComponentBeginOverlap`
  (params (OverlappedComponent :type "PrimitiveComponent Object Reference") (OtherActor :type "Actor Object Reference") (OtherComp :type "PrimitiveComponent Object Reference") (OtherBodyIndex :type Integer) (bFromSweep :type Boolean) (SweepResult :type "HitResult Structure (by ref)"))
  (bind _outactors (`GameplayStatics.GetAllActorsOfClass` "/Game/BP_MoonFloristCharacter.BP_MoonFloristCharacter_C"))
  (if (== OtherActor (`|GetArrayItem` _outactors))
    (bind _outactors_2 (`GameplayStatics.GetAllActorsOfClass` "/Script/MoonFlorist.MyGameManager"))
    (bind _output_get (set `self.GameManager` (`|GetArrayItem` _outactors_2)))
    (`MyGameManager.AddNotification` _output_get (`self.Notification`) (`self.Time`))
    (`self.K2_DestroyActor`)))

(fn `UserConstructionScript`)