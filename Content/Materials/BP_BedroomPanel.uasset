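; Bedroom panel Blueprint that works as a digital clock showing the machine's current local time.
; Tick writes the hour and minute from Now into separate Hour and Minutes text components as two-digit values.
; BeginPlay gives both components dynamic instances of an emissive font material, tinted warm amber.
; An alternative blue tint and a combined hour:minute format remain in the graph but are disconnected.
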(event `self.ReceiveTick`
  (params (DeltaSeconds :type "Float (single-precision)"))
  (bind (_returnvalue_year _returnvalue_month _returnvalue_day _returnvalue_hour _returnvalue_minute) (`KismetMathLibrary.BreakDateTime` (`KismetMathLibrary.Now`)))
  (`TextRenderComponent.K2_SetText` (`self.Hour`) (`KismetTextLibrary.Conv_IntToText` _returnvalue_hour false true 2))
  (`TextRenderComponent.K2_SetText` (`self.Minutes`) (`KismetTextLibrary.Conv_IntToText` _returnvalue_minute false true 2)))

(event `self.ReceiveBeginPlay`
  (bind _returnvalue (`PrimitiveComponent.CreateDynamicMaterialInstance` (`self.Minutes`) 0 "/Game/MI_PepeEmissiveFont.MI_PepeEmissiveFont" "None"))
  (bind _returnvalue_2 (`PrimitiveComponent.CreateDynamicMaterialInstance` (`self.Hour`) 0 "/Game/MI_PepeEmissiveFont.MI_PepeEmissiveFont" "None"))
  (`MaterialInstanceDynamic.SetVectorParameterValue` _returnvalue "Emission Color 01" (struct :`R` 0.723958 :`G` 0.441153 :`B` 0.170204 :`A` 1.0))
  (`MaterialInstanceDynamic.SetVectorParameterValue` _returnvalue_2 "Emission Color 01" (struct :`R` 0.723958 :`G` 0.441153 :`B` 0.170204 :`A` 1.0))
  (`MaterialInstanceDynamic.SetVectorParameterValue` _returnvalue_2 "Emission Color 02" (struct :`R` 0.734375 :`G` 0.37886 :`B` 0.038248 :`A` 1.0))
  (`MaterialInstanceDynamic.SetVectorParameterValue` _returnvalue "Emission Color 02" (struct :`R` 0.734375 :`G` 0.37886 :`B` 0.038248 :`A` 1.0)))

(fn `UserConstructionScript`)